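; Selection pawn for a networked game, letting a player choose a character and flag themselves ready with a gamepad.
; On the remote side, left-stick X steps Charanum in BP_GameInstance between two choices.
; The right face button passes the instance's PlayerID to a Ready event, which sets that slot in BP_GameState's ReadyStruct, then prints TeamID.
; The loop over ReadyStruct after that is empty.
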(event `InputAxisKey|Gamepad_LeftX`
  (params (AxisValue :type "Float (single-precision)"))
  (`/Engine/EditorBlueprintResources/ActorMacros.Switch Has Authority`
    (:`Remote`
      (if (!= AxisValue 0.0)
        (if (> AxisValue 0.0)
          (bind _asbp_game_instance (cast `/Game/GameAssets/BluePrint/GameInstance/BP_GameInstance` (`GameplayStatics.GetGameInstance`)))
          (bind _charanum (`/Game/GameAssets/BluePrint/GameInstance/BP_GameInstance.charanum` _asbp_game_instance))
          (if (< _charanum 1)
            (set `/Game/GameAssets/BluePrint/GameInstance/BP_GameInstance.charanum` (+ _charanum 1) _asbp_game_instance))
          (else
            (bind _asbp_game_instance_2 (cast `/Game/GameAssets/BluePrint/GameInstance/BP_GameInstance` (`GameplayStatics.GetGameInstance`)))
            (bind _charanum_2 (`/Game/GameAssets/BluePrint/GameInstance/BP_GameInstance.charanum` _asbp_game_instance_2))
            (if (> _charanum_2 0)
              (set `/Game/GameAssets/BluePrint/GameInstance/BP_GameInstance.charanum` (- _charanum_2 1) _asbp_game_instance_2))))))))

(event `Ready?`
  (params (id :type Integer))
  (bind _asbp_game_state (cast `/Game/GameAssets/BluePrint/GameState/BP_GameState` (`GameplayStatics.GetGameState`)))
  (`KismetArrayLibrary.Array_Set` (`/Game/GameAssets/BluePrint/GameState/BP_GameState.ReadyStruct` _asbp_game_state) id true)
  (bind _asbp_game_state_2 (cast `/Game/GameAssets/BluePrint/GameState/BP_GameState` (`GameplayStatics.GetGameState`)))
  (for _ (`/Game/GameAssets/BluePrint/GameState/BP_GameState.ReadyStruct` _asbp_game_state_2)
    _))

(event `Key|Gamepad_FaceButton_Right`
  (params (Key :type "Key Structure"))
  (:`Pressed`
    (bind _asbp_game_instance (cast `/Game/GameAssets/BluePrint/GameInstance/BP_GameInstance` (`GameplayStatics.GetGameInstance`)))
    (`self.Ready?` (`/Game/GameAssets/BluePrint/GameInstance/BP_GameInstance.PlayerID` _asbp_game_instance))
    (bind _asbp_game_instance_2 (cast `/Game/GameAssets/BluePrint/GameInstance/BP_GameInstance` (`GameplayStatics.GetGameInstance`)))
    (`KismetSystemLibrary.PrintString` (`KismetStringLibrary.Conv_IntToString` (`/Game/GameAssets/BluePrint/GameInstance/BP_GameInstance.TeamID` _asbp_game_instance_2)))))

(fn `UserConstructionScript`)