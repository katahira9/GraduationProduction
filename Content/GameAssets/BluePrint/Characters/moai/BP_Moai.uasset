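; Playable Moai character (MAI) with two attacks, two specials and a gauge-based ultimate, built around deployable turrets.
; Attack1 fires a target-aimed beam, Special1 deploys turrets capped by recycling the oldest, and Special2 spawns a shield.
; Attack2 makes all MAI-tagged turrets fire at staggered intervals, while the ultimate gives deployed and extra-spawned turrets evenly spaced angles.
; Separate events, gated by DoOnce, trigger spawns after animations start.
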(event `InputAction|Attack1`
  (params (Key :type "Key Structure"))
  ;[1 1 1] Attack1
  (:`Pressed`
    (bind _success (`self.Is Can Use Weapon` "NewEnumerator0"))
    (if _success
      (`self.MAIAttack1Action`))))

(event `InputAction|Attack2`
  (params (Key :type "Key Structure"))
  ;[1 1 1] Attack2
  (:`Pressed`
    (bind _success (`self.Is Can Use Weapon` "NewEnumerator1"))
    (if _success
      (`self.MAIAttack2Action`)
      (`self.DoOnesResetToAttack2`))))

(event `self.ReceiveBeginPlay`
  ;[1 1 1] BeginPlay
  (`parent.ReceiveBeginPlay`)
  (`|ExecutionSequence`
    (:`then_0`
      (`self.SetCharacterStruct` "MAI"))))

(event `MAIAttack2Action`
  ;[1 1 1] Attack2
  (`/Engine/EditorBlueprintResources/StandardMacros.DoOnce` false :!label _label
    (:`Completed`
      (`self.LostAmmo` "NewEnumerator1")
      (`self.InflictWeaponCoolTime` "NewEnumerator1")
      (`self.Attack2Order`))))

(event `MAIAttack1Action`
  ;[1 1 1] Attack1
  (`self.SetStopVelocty` true)
  (`self.SetAnimationServer` "NewEnumerator12")
  (`self.SetMuzzleCorrectionServer` true)
  (`self.GuidedCheck`)
  (goto _label_2 :!via `Reset`))

(event `DoOnesResetToAttack2`
  ;[1 1 1] Attack2
  (goto _label :!via `Reset`))

(event `MAIAttack1Server`
  ;[1 1 1] Attack1
  (`/Engine/EditorBlueprintResources/StandardMacros.DoOnce` false :!label _label_2
    (:`Completed`
      (`self.LostAmmo` "NewEnumerator0")
      (`self.InflictWeaponCoolTime` "NewEnumerator0")
      (`self.MAIAttack1Shot` (`SceneComponent.K2_GetComponentToWorld` (`self.ShotPoint`))))))

(event `MAIAttack2Shot`
  (params (ShotPoint :type "Vector Structure"))
  ;[1 1 1] Attack2
  (`self.Attack2Shot` ShotPoint))

(event `self.ReceiveTick`
  (params (DeltaSeconds :type "Float (single-precision)"))
  ;[1 1 1] Tick
  (`parent.ReceiveTick` DeltaSeconds)
  (`|ExecutionSequence`
    (:`then_0`
      (`self.MoaiJrLiquidation`))))

(event `InputAction|Special1`
  (params (Key :type "Key Structure"))
  ;[1 1 1] Special1
  (:`Pressed`
    (bind _success (`self.Is Can Use Weapon` "NewEnumerator2"))
    (if _success
      (`self.MAISpecial1Action`))))

(event `InputAction|Special2`
  (params (Key :type "Key Structure"))
  ;[1 1 1] Special2
  (:`Pressed`
    (bind _success (`self.Is Can Use Weapon` "NewEnumerator3"))
    (if _success
      (`self.MAISpecial2Action`))))

(event `MAISpecial1Action`
  ;[1 1 1] Special1
  (`self.SetStopVelocty` true)
  (`self.SetAnimationServer` "NewEnumerator13")
  (`self.SetMuzzleCorrectionServer` true)
  (`self.GuidedCheck`)
  (goto _label_3 :!via `Reset`))

(event `MAISpecial2Action`
  ;[1 1 1] Special2
  (`self.SetStopVelocty` true)
  (`self.SetAnimationServer` "NewEnumerator8")
  (`self.GuidedCheck`)
  (goto _label_4 :!via `Reset`))

(event `MAISpecial1Shot`
  ;[1 1 1] Special1
  (`/Engine/EditorBlueprintResources/StandardMacros.DoOnce` false :!label _label_3
    (:`Completed`
      (`self.LostAmmo` "NewEnumerator2")
      (`self.InflictWeaponCoolTime` "NewEnumerator2")
      (`self.Special1Shot`))))

(event `MAISpecial2Shot`
  ;[1 1 1] Special2
  (`/Engine/EditorBlueprintResources/StandardMacros.DoOnce` false :!label _label_4
    (:`Completed`
      (`self.LostAmmo` "NewEnumerator3")
      (`self.InflictWeaponCoolTime` "NewEnumerator3")
      (`self.Special2Shot`))))

(event `MoaiJrAttachMulti`
  ;[1 1 1] Special1
  (`SceneComponent.K2_AttachToComponent` (`self.Mesh_Jr`) (`self.Mesh`) "moaiJr_socket" "KeepRelative" "KeepRelative" "KeepRelative" false))

(event `MoaiJrAttach`
  ;[1 1 1] Special1
  (`self.MoaiJrAttachMulti`))

(event `MoaiJrDettachMulti`
  ;[1 1 1] Special1
  (`SceneComponent.K2_AttachToComponent` (`self.Mesh_Jr`) (`self.Mesh`) "moaiJr_noattach" "KeepRelative" "KeepRelative" "KeepRelative" false))

(event `MoaiJrDettach`
  ;[1 1 1] Special1
  (`self.MoaiJrDettachMulti`))

(event `InputAction|ULT`
  (params (Key :type "Key Structure"))
  ;[1 1 1] ULT
  (:`Pressed`
    (if (>= (`self.ULTGage`) 100.0)
      (bind _success (`self.Is Can Use Weapon` "NewEnumerator4"))
      (if _success
        (`self.MAIULTAction`)))))

(event `MAIULTAction`
  ;[1 1 1] ULT
  (`self.SetStopVelocty` true)
  (`self.SetAnimationServer` "NewEnumerator14")
  (`self.SetMuzzleCorrectionServer` true)
  (`self.GuidedCheck`)
  (set `self.ULTGage` 0.0)
  (`self.ULTOrder` :!label _label_5))

(event `MAIULTOder`
  ;[1 1 1] ULT
  (`/Engine/EditorBlueprintResources/StandardMacros.DoOnce` false
    (:`Completed`
      (goto _label_5))))

(event `MAIULTShot`
  (params (ShotPoint :type "Vector Structure"))
  ;[1 1 1] ULT
  (`self.ULTShot` ShotPoint))

(event `MAIULTMoaiSpawn`
  ;[1 1 1] ULT
  (`self.ULTMoaiSpawn`))

(fn `Attack2Order`
  (locals (FireTime :type "Float (double-precision)" :default 1.0) (FireInterval :type "Float (double-precision)"))
  (bind _outactors (`GameplayStatics.GetAllActorsWithTag` "MAI_Turret"))
  (for (_array_element _array_index) _outactors
    (bind _asbp_turret_mai (cast `/Game/GameAssets/BluePrint/Bullets/Turret/BP_Turret_MAI` _array_element))
    (set `/Game/GameAssets/BluePrint/Bullets/Turret/BP_Turret_MAI.FireTimer` (+ (`local.FireTime`) (* _array_index (`local.FireInterval`))) _asbp_turret_mai)
    (`/Game/GameAssets/BluePrint/Bullets/Turret/BP_Turret_MAI.FireOderServer` _asbp_turret_mai)))

(fn `Attack2Shot`
  (params (ShotPoint :type "Vector Structure"))
  (bind _target (`self.Target`))
  (bind _returnvalue (`self.GetActorForwardVector` (`GameplayStatics.GetPlayerController` 0)))
  (bind _returnvalue_2 (`|SpawnActorFromClass` "/Game/GameAssets/BluePrint/Bullets/Beam/BP_test_beam.BP_test_beam_C" (`KismetMathLibrary.Conv_VectorToTransform` ShotPoint) "Undefined" "OverrideRootScale" null null))
  (`self.FireSeting` _returnvalue_2)
  (`|ExecutionSequence`
    (:`then_0`
      (`/Game/GameAssets/BluePrint/Method/BP_MacroLibrary.IsTargetExistence` _target
        (:`NotExistence`
          (`self.K2_SetActorRotation` _returnvalue_2 (`self.K2_GetActorRotation`) false))
        (:`Existence`
          (bind _returnvalue_3 (`KismetMathLibrary.FindLookAtRotation` (`self.K2_GetActorLocation` _returnvalue_2) (`self.K2_GetActorLocation` (`self.Target`))))
          (`self.K2_SetActorRotation` _returnvalue_2 _returnvalue_3 false)
          (set `/Game/GameAssets/BluePrint/Bullets/BP_BuletBase.MoveDirection` _returnvalue _returnvalue_2)
          (set `/Game/GameAssets/BluePrint/Bullets/BP_BuletBase.Target` (`self.Target`) _returnvalue_2))))
    (:`then_1`
      (`/Game/GameAssets/BluePrint/Method/BP_MacroLibrary.IsTargetExistence` _target
        (:`NotExistence`
          (`/Game/GameAssets/BluePrint/Bullets/BP_BuletBase.SetMoveRotationMulti` _returnvalue_2 (`self.K2_GetActorRotation`))
          (`/Game/GameAssets/BluePrint/Bullets/BP_BuletBase.SetMoveDirectionMulti` _returnvalue_2 _returnvalue))
        (:`Existence`
          (`/Game/GameAssets/BluePrint/Bullets/BP_BuletBase.SetMoveRotationMulti` _returnvalue_2 _returnvalue_3)
          (`/Game/GameAssets/BluePrint/Bullets/BP_BuletBase.SetMoveDirectionMulti` _returnvalue_2 (`KismetMathLibrary.GetForwardVector` _returnvalue_3)))))
    (:`then_2`
      (`self.SetDamageProcess` _returnvalue_2 "NewEnumerator1"))))

(fn `MAIAttack1Shot`
  (params (SpawnTransform :type "Transform Structure"))
  (bind _target (`self.Target`))
  (bind _returnvalue (`self.GetActorForwardVector` (`GameplayStatics.GetPlayerController` 0)))
  (bind _returnvalue_2 (`|SpawnActorFromClass` "/Game/GameAssets/BluePrint/Bullets/Beam/BP_test_beam.BP_test_beam_C" SpawnTransform "Undefined" "OverrideRootScale" null null))
  (`self.FireSeting` _returnvalue_2)
  (`|ExecutionSequence`
    (:`then_0`
      (`/Game/GameAssets/BluePrint/Method/BP_MacroLibrary.IsTargetExistence` _target
        (:`NotExistence`
          (`self.K2_SetActorRotation` _returnvalue_2 (`self.K2_GetActorRotation`) false))
        (:`Existence`
          (bind _returnvalue_3 (`KismetMathLibrary.FindLookAtRotation` (`self.K2_GetActorLocation` _returnvalue_2) (`self.K2_GetActorLocation` (`self.Target`))))
          (`self.K2_SetActorRotation` _returnvalue_2 _returnvalue_3 false)
          (set `/Game/GameAssets/BluePrint/Bullets/BP_BuletBase.MoveDirection` _returnvalue _returnvalue_2)
          (set `/Game/GameAssets/BluePrint/Bullets/BP_BuletBase.Target` (`self.Target`) _returnvalue_2))))
    (:`then_1`
      (`/Game/GameAssets/BluePrint/Method/BP_MacroLibrary.IsTargetExistence` _target
        (:`NotExistence`
          (`/Game/GameAssets/BluePrint/Bullets/BP_BuletBase.SetMoveRotationMulti` _returnvalue_2 (`self.K2_GetActorRotation`))
          (`/Game/GameAssets/BluePrint/Bullets/BP_BuletBase.SetMoveDirectionMulti` _returnvalue_2 _returnvalue))
        (:`Existence`
          (`/Game/GameAssets/BluePrint/Bullets/BP_BuletBase.SetMoveRotationMulti` _returnvalue_2 _returnvalue_3)
          (`/Game/GameAssets/BluePrint/Bullets/BP_BuletBase.SetMoveDirectionMulti` _returnvalue_2 (`KismetMathLibrary.GetForwardVector` _returnvalue_3)))))
    (:`then_2`
      (`self.SetDamageProcess` _returnvalue_2)
      (`self.SetActorScale3D` _returnvalue_2 (5.0 5.0 5.0)))))

(fn `MoaiJrLiquidation`
  (bind _turretmoais (`self.TurretMoais`))
  (bind (_arrayindex _arrayelement) (`/Engine/EditorBlueprintResources/StandardMacros.ReverseForEachLoop` _turretmoais)
    (:`LoopBody`
      (`/Engine/EditorBlueprintResources/StandardMacros.IsValid` _arrayelement
        (:`Is Not Valid`
          (`KismetArrayLibrary.Array_Remove` _turretmoais _arrayindex))))))

(fn `Special1Shot`
  (bind _turretmoais (`self.TurretMoais`))
  (bind _target (`self.Target`))
  (bind _returnvalue (`|SpawnActorFromClass` "/Game/GameAssets/BluePrint/Bullets/Turret/BP_Turret_MAI.BP_Turret_MAI_C" (`KismetMathLibrary.Conv_VectorToTransform` (`SceneComponent.GetSocketLocation` (`self.Mesh`) "moaiJr_spawnPoint")) "Undefined" "OverrideRootScale" null null))
  (`self.FireSeting` _returnvalue)
  (`|ExecutionSequence`
    (:`then_0`
      (`/Game/GameAssets/BluePrint/Method/BP_MacroLibrary.IsTargetExistence` _target
        (:`NotExistence`
          (`self.K2_SetActorRotation` _returnvalue (`self.K2_GetActorRotation`) false))
        (:`Existence`
          (`self.K2_SetActorRotation` (`self.K2_GetActorRotation`))
          (set `/Game/GameAssets/BluePrint/Bullets/BP_BuletBase.Target` (`self.Target`) _returnvalue))))
    (:`then_1`
      (`/Game/GameAssets/BluePrint/Method/BP_MacroLibrary.IsTargetExistence` _target
        (:`NotExistence`
          (`/Game/GameAssets/BluePrint/Bullets/BP_BuletBase.SetMoveRotationMulti` _returnvalue (`self.K2_GetActorRotation`))
          (`/Game/GameAssets/BluePrint/Bullets/BP_BuletBase.SetMoveDirectionMulti` _returnvalue (`self.GetActorForwardVector` (`GameplayStatics.GetPlayerController` 0))))
        (:`Existence`
          (bind _returnvalue_2 (`KismetMathLibrary.FindLookAtRotation` (`self.K2_GetActorLocation` _returnvalue) (`self.K2_GetActorLocation` (`self.Target`))))
          (`/Game/GameAssets/BluePrint/Bullets/BP_BuletBase.SetMoveRotationMulti` _returnvalue _returnvalue_2)
          (`/Game/GameAssets/BluePrint/Bullets/BP_BuletBase.SetMoveDirectionMulti` _returnvalue (`KismetMathLibrary.GetForwardVector` _returnvalue_2)))))
    (:`then_2`
      (`self.SetDamageProcess` _returnvalue "NewEnumerator4"))
    (:`then_3`
      (if (>= (`KismetArrayLibrary.Array_Length` _turretmoais) (`self.MaxMoai`))
        (`self.K2_DestroyActor` (`|GetArrayItem` _turretmoais))
        (`KismetArrayLibrary.Array_Remove` _turretmoais)
        (`KismetArrayLibrary.Array_Add` _turretmoais _returnvalue)
        (else
          (`KismetArrayLibrary.Array_Add` _turretmoais _returnvalue))))))

(fn `Special2Shot`
  (bind _target (`self.Target`))
  (bind _returnvalue (`|SpawnActorFromClass` "/Game/GameAssets/BluePrint/Bullets/Shield/BP_Shield_MAI.BP_Shield_MAI_C" (`KismetMathLibrary.Conv_VectorToTransform` (- (`self.K2_GetActorLocation`) (0.0 0.0 200.0))) "Undefined" "OverrideRootScale" null null))
  (`self.FireSeting` _returnvalue)
  (`|ExecutionSequence`
    (:`then_0`
      (`/Game/GameAssets/BluePrint/Method/BP_MacroLibrary.IsTargetExistence` _target
        (:`NotExistence`
          (`self.K2_SetActorRotation` _returnvalue (`self.K2_GetActorRotation`) false))
        (:`Existence`
          (`self.K2_SetActorRotation` (`self.K2_GetActorRotation`))
          (set `/Game/GameAssets/BluePrint/Bullets/BP_BuletBase.Target` (`self.Target`) _returnvalue))))
    (:`then_1`
      (`/Game/GameAssets/BluePrint/Method/BP_MacroLibrary.IsTargetExistence` _target
        (:`NotExistence`
          (`/Game/GameAssets/BluePrint/Bullets/BP_BuletBase.SetMoveRotationMulti` _returnvalue (`self.K2_GetActorRotation`))
          (`/Game/GameAssets/BluePrint/Bullets/BP_BuletBase.SetMoveDirectionMulti` _returnvalue (`self.GetActorForwardVector` (`GameplayStatics.GetPlayerController` 0))))
        (:`Existence`
          (bind _returnvalue_2 (`KismetMathLibrary.FindLookAtRotation` (`self.K2_GetActorLocation` _returnvalue) (`self.K2_GetActorLocation` (`self.Target`))))
          (`/Game/GameAssets/BluePrint/Bullets/BP_BuletBase.SetMoveRotationMulti` _returnvalue _returnvalue_2)
          (`/Game/GameAssets/BluePrint/Bullets/BP_BuletBase.SetMoveDirectionMulti` _returnvalue (`KismetMathLibrary.GetForwardVector` _returnvalue_2)))))
    (:`then_2`
      (`self.SetDamageProcess` _returnvalue "NewEnumerator3"))))

(fn `ULTMoaiSpawn`
  (bind _target (`self.Target`))
  (bind _target_2 (`self.Target`))
  (bind _returnvalue (`self.GetActorForwardVector` (`GameplayStatics.GetPlayerController` 0)))
  (bind _returnvalue_2 (`self.GetActorForwardVector` (`GameplayStatics.GetPlayerController` 0)))
  (`|ExecutionSequence`
    (:`then_0`
      (bind _returnvalue_3 (`|SpawnActorFromClass` "/Game/GameAssets/BluePrint/Bullets/Turret/BP_Turret_MAI.BP_Turret_MAI_C" (`KismetMathLibrary.Conv_VectorToTransform` (`SceneComponent.GetSocketLocation` (`self.Mesh`) "spawnPoint1")) "Undefined" "OverrideRootScale" null null))
      (`self.FireSeting` _returnvalue_3)
      (`|ExecutionSequence`
        (:`then_0`
          (`/Game/GameAssets/BluePrint/Method/BP_MacroLibrary.IsTargetExistence` _target
            (:`NotExistence`
              (`self.K2_SetActorRotation` _returnvalue_3 (`self.K2_GetActorRotation`) false))
            (:`Existence`
              (bind _returnvalue_4 (`KismetMathLibrary.FindLookAtRotation` (`self.K2_GetActorLocation` _returnvalue_3) (`self.K2_GetActorLocation` (`self.Target`))))
              (`self.K2_SetActorRotation` _returnvalue_3 _returnvalue_4 false)
              (set `/Game/GameAssets/BluePrint/Bullets/BP_BuletBase.MoveDirection` _returnvalue _returnvalue_3)
              (set `/Game/GameAssets/BluePrint/Bullets/BP_BuletBase.Target` (`self.Target`) _returnvalue_3))))
        (:`then_1`
          (`/Game/GameAssets/BluePrint/Method/BP_MacroLibrary.IsTargetExistence` _target
            (:`NotExistence`
              (`/Game/GameAssets/BluePrint/Bullets/BP_BuletBase.SetMoveRotationMulti` _returnvalue_3 (`self.K2_GetActorRotation`))
              (`/Game/GameAssets/BluePrint/Bullets/BP_BuletBase.SetMoveDirectionMulti` _returnvalue_3 _returnvalue))
            (:`Existence`
              (`/Game/GameAssets/BluePrint/Bullets/BP_BuletBase.SetMoveRotationMulti` _returnvalue_3 _returnvalue_4)
              (`/Game/GameAssets/BluePrint/Bullets/BP_BuletBase.SetMoveDirectionMulti` _returnvalue_3 (`KismetMathLibrary.GetForwardVector` _returnvalue_4)))))
        (:`then_2`
          (`self.SetDamageProcess` _returnvalue_3 "NewEnumerator4")
          (`KismetArrayLibrary.Array_Add` (`self.ULTMoais`) _returnvalue_3))))
    (:`then_1`
      (bind _returnvalue_5 (`|SpawnActorFromClass` "/Game/GameAssets/BluePrint/Bullets/Turret/BP_Turret_MAI.BP_Turret_MAI_C" (`KismetMathLibrary.Conv_VectorToTransform` (`SceneComponent.GetSocketLocation` (`self.Mesh`) "spawnPoint2")) "Undefined" "OverrideRootScale" null null))
      (`self.FireSeting` _returnvalue_5)
      (`|ExecutionSequence`
        (:`then_0`
          (`/Game/GameAssets/BluePrint/Method/BP_MacroLibrary.IsTargetExistence` _target_2
            (:`NotExistence`
              (`self.K2_SetActorRotation` _returnvalue_5 (`self.K2_GetActorRotation`) false))
            (:`Existence`
              (bind _returnvalue_6 (`KismetMathLibrary.FindLookAtRotation` (`self.K2_GetActorLocation` _returnvalue_5) (`self.K2_GetActorLocation` (`self.Target`))))
              (`self.K2_SetActorRotation` _returnvalue_5 _returnvalue_6 false)
              (set `/Game/GameAssets/BluePrint/Bullets/BP_BuletBase.MoveDirection` _returnvalue_2 _returnvalue_5)
              (set `/Game/GameAssets/BluePrint/Bullets/BP_BuletBase.Target` (`self.Target`) _returnvalue_5))))
        (:`then_1`
          (`/Game/GameAssets/BluePrint/Method/BP_MacroLibrary.IsTargetExistence` _target_2
            (:`NotExistence`
              (`/Game/GameAssets/BluePrint/Bullets/BP_BuletBase.SetMoveRotationMulti` _returnvalue_5 (`self.K2_GetActorRotation`))
              (`/Game/GameAssets/BluePrint/Bullets/BP_BuletBase.SetMoveDirectionMulti` _returnvalue_5 _returnvalue_2))
            (:`Existence`
              (`/Game/GameAssets/BluePrint/Bullets/BP_BuletBase.SetMoveRotationMulti` _returnvalue_5 _returnvalue_6)
              (`/Game/GameAssets/BluePrint/Bullets/BP_BuletBase.SetMoveDirectionMulti` _returnvalue_5 (`KismetMathLibrary.GetForwardVector` _returnvalue_6)))))
        (:`then_2`
          (`self.SetDamageProcess` _returnvalue_5 "NewEnumerator4")
          (`KismetArrayLibrary.Array_Add` (`self.ULTMoais`)))))))

(fn `ULTOrder`
  (locals (DelayTime :type "Float (double-precision)") (AddDelay :type "Float (double-precision)"))
  (`|ExecutionSequence`
    (:`then_0`
      (for _array_element (`self.TurretMoais`)
        (`KismetArrayLibrary.Array_Add` (`self.ULTMoais`) _array_element))
      (`KismetArrayLibrary.Array_Clear` (`self.TurretMoais`)))
    (:`then_1`
      (for (_array_element_2 _array_index) (`self.ULTMoais`)
        (set `/Game/GameAssets/BluePrint/Bullets/BP_BuletBase.bisULT` true _array_element_2)
        (set `/Game/GameAssets/BluePrint/Bullets/Turret/BP_Turret_MAI.ULTAngle` (* _array_index (/ 360.0 (`KismetMathLibrary.Conv_IntToDouble` (`KismetArrayLibrary.Array_Length` (`self.ULTMoais`))))) _array_element_2)
        (set `/Game/GameAssets/BluePrint/Bullets/Turret/BP_Turret_MAI.ULTTimer` 10.0 _array_element_2)
        (set `/Game/GameAssets/BluePrint/Bullets/Turret/BP_Turret_MAI.ULTStandbyTimer` 1.0 _array_element_2))
      (`KismetArrayLibrary.Array_Clear` (`self.ULTMoais`)))))

(fn `ULTShot`
  (params (ShotPoint :type "Vector Structure"))
  (bind _target (`self.Target`))
  (bind _returnvalue (`self.GetActorForwardVector` (`GameplayStatics.GetPlayerController` 0)))
  (bind _returnvalue_2 (`|SpawnActorFromClass` "/Game/GameAssets/BluePrint/Bullets/Beam/BP_test_beam.BP_test_beam_C" (`KismetMathLibrary.Conv_VectorToTransform` ShotPoint) "Undefined" "OverrideRootScale" null null))
  (`self.FireSeting` _returnvalue_2)
  (`|ExecutionSequence`
    (:`then_0`
      (`/Game/GameAssets/BluePrint/Method/BP_MacroLibrary.IsTargetExistence` _target
        (:`NotExistence`
          (`self.K2_SetActorRotation` _returnvalue_2 (`self.K2_GetActorRotation`) false))
        (:`Existence`
          (bind _returnvalue_3 (`KismetMathLibrary.FindLookAtRotation` (`self.K2_GetActorLocation` _returnvalue_2) (`self.K2_GetActorLocation` (`self.Target`))))
          (`self.K2_SetActorRotation` _returnvalue_2 _returnvalue_3 false)
          (set `/Game/GameAssets/BluePrint/Bullets/BP_BuletBase.MoveDirection` _returnvalue _returnvalue_2)
          (set `/Game/GameAssets/BluePrint/Bullets/BP_BuletBase.Target` (`self.Target`) _returnvalue_2))))
    (:`then_1`
      (`/Game/GameAssets/BluePrint/Method/BP_MacroLibrary.IsTargetExistence` _target
        (:`NotExistence`
          (`/Game/GameAssets/BluePrint/Bullets/BP_BuletBase.SetMoveRotationMulti` _returnvalue_2 (`self.K2_GetActorRotation`))
          (`/Game/GameAssets/BluePrint/Bullets/BP_BuletBase.SetMoveDirectionMulti` _returnvalue_2 _returnvalue))
        (:`Existence`
          (`/Game/GameAssets/BluePrint/Bullets/BP_BuletBase.SetMoveRotationMulti` _returnvalue_2 _returnvalue_3)
          (`/Game/GameAssets/BluePrint/Bullets/BP_BuletBase.SetMoveDirectionMulti` _returnvalue_2 (`KismetMathLibrary.GetForwardVector` _returnvalue_3)))))
    (:`then_2`
      (`self.SetDamageProcess` _returnvalue_2 "NewEnumerator4"))))

(fn `UserConstructionScript`
  (`parent.UserConstructionScript`))