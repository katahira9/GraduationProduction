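; Playable Itukusima (ITK) character, extending a base character with two socket-attached funnels that launch at the target via Special1.
; Melee inputs start a timed, boost-draining homing dash or, at close range, trigger Gameplay Ability System attacks by tag.
; Tick drives that dash and derives the movement, step and damage state enum.
; Death deducts team cost and hides the funnels until respawn; beam-shot logic exists but is largely disconnected.
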(event `OnEntryCombat1`
  ;[1 0 0.3542] マージ
  (set `self.bIsEntryCombat1` true))

(event `OffEntryCombat1`
  ;[1 0 0.3542] マージ
  (set `self.bIsEntryCombat1` false))

(event `OnEntryCombat2`
  ;[1 0 0.3542] マージ
  (set `self.bIsEntryCombat2` true))

(event `OffEntryCombat2`
  ;[1 0 0.3542] マージ
  (set `self.bIsEntryCombat2` false))

(event `OnCombat`
  ;[1 0 0.3542] マージ
  (set `self.bIsCombat` true))

(event `OffCombat`
  ;[1 0 0.3542] マージ
  (set `self.bIsCombat` false))

(event `OnFirstAttack`
  ;[1 0 0.3542] マージ
  (set `self.bIsFirstAttack` true))

(event `OffFirstAttack`
  ;[1 0 0.3542] マージ
  (set `self.bIsFirstAttack` false))

(event `ConbatTimerServer`
  ;[1 0 0.3542] マージ
  (bind _outtimer (`self.Conbat Timer`))
  (if (<= _outtimer 0.0)
    (set `self.bIsGuideEnd` true)
    (else
      (set `self.bIsGuideEnd` false))))

(event `SetGuideTimerServer`
  (params (Time :type "Float (double-precision)"))
  ;[1 0 0.3542] マージ
  (set `self.Guide_Timer` Time))

(event `SetGuideEnd`
  (params (NewParam :type Boolean))
  ;[1 0 0.3542] マージ
  (set `self.bIsGuideEnd` NewParam))

(event `RightFunnelSpwanServer`
  ;[1 1 1] ファンネルをスポーン
  (if (== (`self.Funnel_Right`) null)
    (bind _returnvalue (`|SpawnActorFromClass` "/Game/GameAssets/BluePrint/Bullets/Funnel/BP_Funnel.BP_Funnel_C" (`KismetMathLibrary.Conv_VectorToTransform` (`SceneComponent.GetSocketLocation` (`self.Mesh`) "funnel_rightSocket")) "Undefined" "OverrideRootScale" null null))
    (set `/Game/GameAssets/BluePrint/Bullets/Funnel/BP_Funnel.Master` self _returnvalue)
    (set `self.Funnel_Right` _returnvalue)
    (set `/Game/GameAssets/BluePrint/Bullets/Funnel/BP_Funnel.AttachSocketName` "funnel_rightSocket" _returnvalue)))

(event `InputAction|Special1`
  (params (Key :type "Key Structure"))
  ;[1 1 1] ファンネル射出
  (:`Pressed`
    (bind _success (`self.Is Can Use Weapon` "NewEnumerator2"))
    (if _success
      (`self.FunnelServer`))))

(event `FunnelServer`
  (bind _funnel_left (`self.Funnel_Left`))
  (bind _funnel_right (`self.Funnel_Right`))
  (bind _returnvalue (`self.K2_GetActorLocation` (`self.Target`)))
  (bind _returnvalue_2 (`self.K2_GetActorLocation` (`self.Target`)))
  (bind _returnvalue_3 (`KismetMathLibrary.FindLookAtRotation` (`self.K2_GetActorLocation` _funnel_right) _returnvalue))
  ;[1 1 1] ファンネル射出
  (`self.LostAmmo` "NewEnumerator2")
  (`self.InflictWeaponCoolTime` "NewEnumerator2")
  (`|ExecutionSequence`
    (:`then_0`
      (`self.SetGuidance` _funnel_right)
      (if (`/Game/GameAssets/BluePrint/Bullets/Funnel/BP_Funnel.IsAttach` _funnel_right)
        (set `/Game/GameAssets/BluePrint/Bullets/Funnel/BP_Funnel.IsAttach` false _funnel_right)
        (`PrimitiveComponent.SetCollisionEnabled` (`/Game/GameAssets/BluePrint/Bullets/BP_BuletBase.DamageCapsule` _funnel_right) "QueryOnly")
        (set `/Game/GameAssets/BluePrint/Bullets/BP_BuletBase.Target` (`self.Target`) _funnel_right)
        (`/Game/GameAssets/BluePrint/Bullets/Funnel/BP_Funnel.LookUp` _funnel_right _returnvalue)
        (set `/Game/GameAssets/BluePrint/Bullets/BP_BuletBase.MoveDirection` (`KismetMathLibrary.GetForwardVector` _returnvalue_3) _funnel_right)
        (set `/Game/GameAssets/BluePrint/Bullets/BP_BuletBase.MoveRotation` _returnvalue_3 _funnel_right)
        (bind _weaponstatus (`self.GetWeaponStatus` "NewEnumerator2"))
        (bind _damagestatus (`self.GetDamageStatus` _weaponstatus))
        (set `/Game/GameAssets/BluePrint/Bullets/BP_BuletBase.DamageStruct` _damagestatus _funnel_right)
        (set `/Game/GameAssets/BluePrint/Bullets/BP_BuletBase.ConsortPlaneValue` (`self.ConsortPlaneValue`) _funnel_right)))
    (:`then_1`
      (`self.SetGuidance` _funnel_left)
      (if (`/Game/GameAssets/BluePrint/Bullets/Funnel/BP_Funnel.IsAttach` _funnel_left)
        (set `/Game/GameAssets/BluePrint/Bullets/Funnel/BP_Funnel.IsAttach` false _funnel_left)
        (`PrimitiveComponent.SetCollisionEnabled` (`/Game/GameAssets/BluePrint/Bullets/BP_BuletBase.DamageCapsule` _funnel_left) "QueryOnly")
        (set `/Game/GameAssets/BluePrint/Bullets/BP_BuletBase.Target` (`self.Target`) _funnel_left)
        (`/Game/GameAssets/BluePrint/Bullets/Funnel/BP_Funnel.LookUp` _funnel_left _returnvalue_2)
        (set `/Game/GameAssets/BluePrint/Bullets/BP_BuletBase.MoveDirection` (`KismetMathLibrary.GetForwardVector` (`KismetMathLibrary.FindLookAtRotation` (`self.K2_GetActorLocation` _funnel_left) _returnvalue_2)) _funnel_left)
        (set `/Game/GameAssets/BluePrint/Bullets/BP_BuletBase.MoveRotation` _returnvalue_3 _funnel_left)
        (bind _weaponstatus_2 (`self.GetWeaponStatus` "NewEnumerator2"))
        (bind _damagestatus_2 (`self.GetDamageStatus` _weaponstatus_2))
        (set `/Game/GameAssets/BluePrint/Bullets/BP_BuletBase.DamageStruct` _damagestatus_2 _funnel_left)
        (set `/Game/GameAssets/BluePrint/Bullets/BP_BuletBase.ConsortPlaneValue` (`self.ConsortPlaneValue`) _funnel_left)))))

(event `self.ReceiveBeginPlay`
  ;[1 1 1] Begin
  (`parent.ReceiveBeginPlay`)
  (`|ExecutionSequence`
    (:`then_0`
      (`self.RightFunnelSpwanServer`)
      (`self.LeftFunnelSpwanServer`))
    (:`then_1`
      (`self.SetCharacterStruct` "ITK"))
    (:`then_2`
      (`KM_GAHelperFunctions.SetupAbilitySystem` null (`self.AbilitySystem`) (`self.Ability List`)))))

(event `LeftFunnelSpwanServer`
  ;[1 1 1] ファンネルをスポーン
  (if (== (`self.Funnel_Left`) null)
    (bind _returnvalue (`|SpawnActorFromClass` "/Game/GameAssets/BluePrint/Bullets/Funnel/BP_Funnel.BP_Funnel_C" (`KismetMathLibrary.Conv_VectorToTransform` (`SceneComponent.GetSocketLocation` (`self.Mesh`) "funnel_leftSocket")) "Undefined" "OverrideRootScale" null null))
    (set `/Game/GameAssets/BluePrint/Bullets/Funnel/BP_Funnel.Master` self _returnvalue)
    (set `self.Funnel_Left` _returnvalue)
    (set `/Game/GameAssets/BluePrint/Bullets/Funnel/BP_Funnel.AttachSocketName` "funnel_leftSocket" _returnvalue)))

(event `self.ReceiveTick`
  (params (DeltaSeconds :type "Float (single-precision)"))
  (bind (_returnvalue_roll _returnvalue_pitch _returnvalue_yaw) (`KismetMathLibrary.BreakRotator` (`self.K2_GetActorRotation`)))
  (bind (_returnvalue_roll_2 _returnvalue_pitch_2 _returnvalue_yaw_2) (`KismetMathLibrary.BreakRotator` (`self.K2_GetActorRotation`)))
  ;[1 1 1] Tick
  (`|ExecutionSequence`
    (:`then_0`
      (`parent.ReceiveTick` DeltaSeconds))
    (:`then_1`
      (if (`self.bIsDamage`)
        (`self.Set_Damage_State`)
        (elif (`self.bIsAttack`)
          _
          (elif (`self.bIsEntryCombat1`)
            (set `self.ItukusimaState` "NewEnumerator8")
            (elif (`self.bIsEntryCombat2`)
              (set `self.ItukusimaState` "NewEnumerator9")
              (elif (`self.bIsBoostDash`)
                (set `self.ItukusimaState` "NewEnumerator1")
                (elif (`self.bJumpKeyDown`)
                  (set `self.ItukusimaState` "NewEnumerator2")
                  (else
                    (set `self.ItukusimaState` "NewEnumerator0")))))))))
    (:`then_2`
      (if (not (`self.bIsDamage`))
        (`self.Set_Step_State`)))
    (:`then_3`
      (if (`self.bIsAttack`)
        (if (not (!= (`self.GetCurrentMontage`) null))
          (set `self.bIsAttack` false))))
    (:`then_4`
      (if (or (`self.bIsEntryCombat1`) (`self.bIsEntryCombat2`))
        _
        (elif (not (!= (`self.GetCurrentMontage`) null))
          (`self.OffCombat`))))
    (:`then_5`
      (`|ExecutionSequence`
        (:`then_1`
          (if (or (`self.bIsEntryCombat2`) (`self.bIsEntryCombat1`) false)
            (if (or (`self.bIsBoostDash`) (`self.bStepping`))
              (`self.OffEntryCombat1`)
              (set `self.bIsEntryCombat1` false)
              (`self.OffEntryCombat2`)
              (set `self.bIsEntryCombat2` false)
              (`self.ResetVelocityServer`)
              (set `self.bDoingCombat2` false)
              (set `self.bCanAttack` false)
              (else
                (`self.FightingGuidanceMove`)
                (set `self.BoostGauge` (- (`self.BoostGauge`) (* (`self.CombatCost`) (`GameplayStatics.GetWorldDeltaSeconds`))))
                (bind _distance (`self.Get Target Distnce`))
                (if (< _distance 130.0)
                  (set `self.bCanAttack` true)
                  (`self.OnFirstAttack`)
                  (if (`self.bIsEntryCombat2`)
                    (set `self.bDoingCombat2` true)
                    (`self.OffEntryCombat2`)
                    (set `self.bIsEntryCombat2` false)
                    (`self.K2_SetActorRotation` (`KismetMathLibrary.MakeRotator` 0.0 0.0 _returnvalue_yaw) :!label _label)
                    (set `self.bCanAttack` true)
                    (elif (`self.bIsEntryCombat1`)
                      (`KismetSystemLibrary.PrintString` "Hello")
                      (`self.OffEntryCombat1`)
                      (set `self.bIsEntryCombat1` false)
                      (goto _label)))
                  (else
                    (set `self.bCanAttack` false)
                    (`self.ConbatTimerServer`)
                    (if (`self.bIsGuideEnd`)
                      (if (`self.bIsEntryCombat1`)
                        (`self.Attack1`)
                        (bind _output_get (set `self.bIsCombatCoolTime` true :!label _label_2))
                        (`self.SetCombatCoolTime` _output_get)
                        (`self.OffEntryCombat2`)
                        (`self.OffEntryCombat1`)
                        (set `self.bIsEntryCombat1` false)
                        (set `self.bIsEntryCombat2` false)
                        (`self.OffCombat`)
                        (set `self.bDoingCombat2` false)
                        (`self.ResetVelocityServer`)
                        (`self.K2_SetActorRotation` (`KismetMathLibrary.MakeRotator` 0.0 0.0 _returnvalue_yaw_2))
                        (elif (`self.bIsEntryCombat2`)
                          (`self.Attack2`)
                          (goto _label_2))))))))))))
    (:`then_6`
      (`|ExecutionSequence`
        (:`then_0`
          (if (`self.bIsCombatCoolTime`)
            (`KismetSystemLibrary.Delay` 1.0)
            (bind _output_get_2 (set `self.bIsCombatCoolTime` false))
            (`self.SetCombatCoolTime` _output_get_2)))
        (:`then_1`
          (if (`self.IsAttacking`)
            (`KismetSystemLibrary.Delay` 3.0)
            (set `self.IsAttacking` false)))))))

(event `Attack2`
  (`self.OnCombat`)
  (set `self.IsAttacking` true)
  (set `self.bIsAttack` true :!label _label_3)
  (`AbilitySystemComponent.TryActivateAbilitiesByTag` (`self.AbilitySystem`) (`BlueprintGameplayTagLibrary.MakeLiteralGameplayTagContainer` (struct :`GameplayTags` (struct :`(TagName` "Attack.B")))) true)
  (`KismetSystemLibrary.PrintString` "Hello")
  (set `self.IsAttacking` false))

(event `InputAction|Attack2`
  (params (Key :type "Key Structure"))
  (:`Pressed`
    (if (not (`self.bIsCombatCoolTime`))
      (`self.OnCombat`)
      (if (`self.bStepping`)
        (`self.Set_Step_State`)
        (else
          (bind _distance (`self.Get Target Distnce`))
          (if (or (< _distance 130.0) (`self.bIsEntryCombat2`))
            (if (`self.bIsFirstAttack`)
              (if (`self.bCanAttack`)
                (if (not (`self.IsAttacking`))
                  (goto _label_3))))
            (elif (not (`self.bIsEntryCombat1`))
              (`self.OnEntryCombat2`)
              (set `self.bIsEntryCombat2` true)
              (`self.SetGuideTimerServer` (`self.FIGHTING_GUIDE_TIME`))
              (`self.SetGuideEnd` false)
              (`self.OffFirstAttack`)))))))
  (:`Released`
    (set `self.bIsAttack` false :!label _label_4)))

(event `Attack1`
  (`KismetSystemLibrary.PrintString` "Hello")
  (set `self.IsAttacking` true)
  (`AbilitySystemComponent.TryActivateAbilitiesByTag` (`self.AbilitySystem`) (`BlueprintGameplayTagLibrary.MakeLiteralGameplayTagContainer` (struct :`GameplayTags` (struct :`(TagName` "Attack.A")))) true :!label _label_5)
  (set `self.IsAttacking` false)
  (`KismetSystemLibrary.PrintString` "Hello"))

(event `InputAction|Attack1`
  (params (Key :type "Key Structure"))
  (:`Pressed`
    (if (not (`self.bIsCombatCoolTime`))
      (`self.OnCombat`)
      (if (`self.bStepping`)
        (`self.Set_Step_State`)
        (else
          (bind _distance (`self.Get Target Distnce`))
          (if (< _distance 130.0)
            (if (`self.bIsFirstAttack`)
              (if (`self.bCanAttack`)
                (set `self.bIsAttack` true)
                (goto _label_5)))
            (elif (not (or (`self.bIsEntryCombat2`) (`self.bIsEntryCombat1`)))
              (`self.OnEntryCombat1`)
              (set `self.bIsEntryCombat1` true)
              (`self.SetGuideTimerServer` (`self.FIGHTING_GUIDE_TIME`))
              (`self.SetGuideEnd` false)
              (`self.OffFirstAttack`)))))))
  (:`Released`
    (goto _label_4)))

(event `BoostDashState`
  (set `self.ItukusimaState` "NewEnumerator1"))

(event `Boost Jump State`
  (set `self.ItukusimaState` "NewEnumerator2"))

(event `Set_Step_State`
  (if (`self.bStepping`)
    (if true
      (`self.StopAnimMontage` (`self.GetCurrentMontage`))
      (set `self.bIsAttack` false))
    (switch `/Game/GameAssets/BluePrint/Characters/StepState` (`self.StepState`)
      (:`NewEnumerator0`
        (set `self.ItukusimaState` "NewEnumerator3"))
      (:`NewEnumerator1`
        (set `self.ItukusimaState` "NewEnumerator4"))
      (:`NewEnumerator2`
        (set `self.ItukusimaState` "NewEnumerator5"))
      (:`NewEnumerator3`
        (set `self.ItukusimaState` "NewEnumerator6")))))

(event `Set_Damage_State`
  (switch `/Game/GameAssets/BluePrint/Enum/EN_DamageReaction` (`self.Damage_Reaction`)
    (:`NewEnumerator1`
      (set `self.ItukusimaState` "NewEnumerator11"))
    (:`NewEnumerator2`
      (set `self.ItukusimaState` "NewEnumerator12"))
    (:`NewEnumerator3`
      (set `self.ItukusimaState` "NewEnumerator13"))))

(event `FireServer`
  (bind _target (`self.Target`))
  (bind _returnvalue (`KismetMathLibrary.FindLookAtRotation` (`self.K2_GetActorLocation`) (`self.K2_GetActorLocation` (`self.Target`))))
  ;[0.2983 0.9302 1] 簡易射撃
  (`self.LostAmmo` "NewEnumerator0")
  (`self.InflictWeaponCoolTime` "NewEnumerator0")
  (bind _returnvalue_2 (`|SpawnActorFromClass` "/Game/GameAssets/BluePrint/Bullets/Beam/BP_test_beam.BP_test_beam_C" (`self.GetTransform`) "Undefined" "OverrideRootScale" null null))
  (`self.FireSeting` _returnvalue_2)
  (`|ExecutionSequence`
    (:`then_0`
      (`/Game/GameAssets/BluePrint/Method/BP_MacroLibrary.IsTargetExistence` _target
        (:`NotExistence`
          (`self.K2_SetActorRotation` _returnvalue_2 (`self.K2_GetActorRotation` (`GameplayStatics.GetPlayerController` 0)) false))
        (:`Existence`
          (`self.K2_SetActorRotation` _returnvalue_2 _returnvalue false)
          (set `/Game/GameAssets/BluePrint/Bullets/BP_BuletBase.Target` (`self.Target`) _returnvalue_2))))
    (:`then_1`
      (`/Game/GameAssets/BluePrint/Method/BP_MacroLibrary.IsTargetExistence` _target
        (:`NotExistence`
          (set `/Game/GameAssets/BluePrint/Bullets/BP_BuletBase.MoveRotation` (`self.K2_GetActorRotation`) _returnvalue_2)
          (set `/Game/GameAssets/BluePrint/Bullets/BP_BuletBase.MoveDirection` (`self.GetActorForwardVector` (`GameplayStatics.GetPlayerController` 0)) _returnvalue_2))
        (:`Existence`
          (set `/Game/GameAssets/BluePrint/Bullets/BP_BuletBase.MoveRotation` _returnvalue _returnvalue_2)
          (set `/Game/GameAssets/BluePrint/Bullets/BP_BuletBase.MoveDirection` (`KismetMathLibrary.GetForwardVector` _returnvalue) _returnvalue_2))))
    (:`then_2`
      (`self.SetDamageProcess` _returnvalue_2))))

(event `InputAction|Attack2`
  (params (Key :type "Key Structure"))
  ;[0.2983 0.9302 1] 簡易射撃
  (:`Pressed`
    (bind _success (`self.Is Can Use Weapon` "NewEnumerator1"))
    (if _success
      (`self.Attack2ITK`))))

(event `Attack2ITK`
  ;[1 1 1] 強射撃
)

(fn `Conbat Timer`
  (returns (OutTimer :type "Float (double-precision)"))
  (bind _output_get (set `self.Guide_Timer` (- (`self.Guide_Timer`) (`GameplayStatics.GetWorldDeltaSeconds`))))
  (return _output_get))

(fn `Damage HP`
  (params (Damage :type "Float (double-precision)") (MinDamage :type "Float (double-precision)"))
  (bind _cost (`self.Cost`))
  (bind _returnvalue (- (`self.HP`) (`KismetMathLibrary.FClamp` (* Damage (`self.DamageCutValue`)) MinDamage 1000.0)))
  (if (<= _returnvalue 0.0)
    (set `self.HP` 0.0)
    (set `self.IsDead` true)
    (`self.GuidedOffPlayer`)
    (`PrimitiveComponent.SetCollisionEnabled` (`self.CapsuleComponent`) "NoCollision")
    (`|ExecutionSequence`
      (:`then_0`
        (`self.SetActorHiddenInGame` true)
        (bind _asbp_game_state (cast `/Game/GameAssets/BluePrint/GameState/BP_GameState` (`GameplayStatics.GetGameState`)))
        (bind _asbp_player_state (cast `/Game/GameAssets/BluePrint/PlayerState/BP_PlayerState` (`self.PlayerState`)))
        (switch `int` (`/Game/GameAssets/BluePrint/PlayerState/BP_PlayerState.TeamID` _asbp_player_state)
          (:`0`
            (set `/Game/GameAssets/BluePrint/GameState/BP_GameState.Team0Cost` (`KismetMathLibrary.FClamp` (- (`/Game/GameAssets/BluePrint/GameState/BP_GameState.Team0Cost` _asbp_game_state) _cost) 0.0 6000.0) _asbp_game_state))
          (:`1`
            (set `/Game/GameAssets/BluePrint/GameState/BP_GameState.Team1Cost` (`KismetMathLibrary.FClamp` (- (`/Game/GameAssets/BluePrint/GameState/BP_GameState.Team1Cost` _asbp_game_state) _cost) 0.0 6000.0) _asbp_game_state))))
      (:`then_1`
        (`self.SetActorHiddenInGame` (`self.Funnel_Right`) true))
      (:`then_2`
        (`self.SetActorHiddenInGame` (`self.Funnel_Left`) true)))
    (elif (== (mod _returnvalue 1.0) 0.0)
      (set `self.HP` (`KismetMathLibrary.FClamp` _returnvalue 0.0 (`self.MaxHP`)))
      (else
        (set `self.HP` (`KismetMathLibrary.FClamp` (`KismetMathLibrary.Conv_IntToDouble` (`KismetMathLibrary.Round` (+ _returnvalue 0.5))) 0.0 (`self.MaxHP`)))))))

(fn `RespawnProcessing`
  (bind _returnvalue (`self.K2_GetActorRotation`))
  (bind _mesh (`self.Mesh`))
  (bind _funnel_right (`self.Funnel_Right`))
  (bind _funnel_left (`self.Funnel_Left`))
  (`parent.RespawnProcessing`)
  (`|ExecutionSequence`
    (:`then_0`
      (if (`KismetSystemLibrary.IsValid` _funnel_right)
        (`self.SetActorHiddenInGame` _funnel_right false)
        (`self.K2_SetActorLocation` _funnel_right (`SceneComponent.GetSocketLocation` _mesh "funnel_rightSocket") false true)
        (`self.K2_SetActorRotation` _funnel_right _returnvalue false)))
    (:`then_1`
      (`/Engine/EditorBlueprintResources/StandardMacros.IsValid` _funnel_left
        (:`Is Valid`
          (`self.SetActorHiddenInGame` _funnel_left false)
          (`self.K2_SetActorLocation` _funnel_left (`SceneComponent.GetSocketLocation` _mesh "funnel_leftSocket") false true)
          (`self.K2_SetActorRotation` _funnel_left _returnvalue false))))))

(fn `UserConstructionScript`
  (`parent.UserConstructionScript`))