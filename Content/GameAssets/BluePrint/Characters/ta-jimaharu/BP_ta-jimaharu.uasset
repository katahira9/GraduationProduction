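; Playable TJM character that fights with four beam funnels and a machine-gun funnel, spawned at mesh sockets on BeginPlay.
; Attack1 fires the MG through Tick while held; Attack2 launches one attached funnel at the target.
; Special1 deploys all four for staggered fire, then recalls them and refills Attack2 ammo; Special2 fires a large beam.
; DoOnce gates delay Attack2 and Special2 shots until separate events trigger them; death and respawn toggle funnel visibility.
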(event `Sp1BeamShot`
  (params (SpawnTransform :type "Transform Structure"))
  ;[1 1 1] BeamShotSp1
  (`self.TJMSp1Bulet` SpawnTransform))

(event `Atk1Shot`
  (params (SpawnTransform :type "Transform Structure"))
  ;[1 1 1] Attack1Shot
  ;;[1 0.4791 0.5792] コメント
  (`self.TJMAtk1Bulet` SpawnTransform))

(event `SetUseMGServer`
  (params (UseMG :type Boolean))
  ;[1 1 1] カスタムイベント
  (set `self.IsUseMG` UseMG))

(event `FunnelSpawnServer`
  ;[1 1 1] カスタムイベント
  (`self.FunnelSpawn`))

(event `UseMGServer`
  ;[1 1 1] MG
  (`self.LostAmmo` "NewEnumerator0")
  (`self.InflictWeaponCoolTime` "NewEnumerator0")
  (bind _shottransform (`self.SearchShotPosition`))
  (`self.Atk1Shot` _shottransform))

(event `self.ReceiveBeginPlay`
  ;[1 1 1] BeginPlay
  (`parent.ReceiveBeginPlay`)
  (`|ExecutionSequence`
    (:`then_0`
      (`self.FunnelSpawnServer`))
    (:`then_1`
      (`self.SetCharacterStruct` "TJM"))
    (:`then_2`
      (set `self.TopCameraPoint` (0.0 0.0 400.0))
      (set `self.AnderCameraPoint` (0.0 0.0 10.0))
      (set `SpringArmComponent.TargetArmLength` 800.0 (`self.CameraBoom`)))))

(event `self.ReceiveTick`
  (params (DeltaSeconds :type "Float (single-precision)"))
  ;[1 1 1] Tick
  (`parent.ReceiveTick` DeltaSeconds)
  (`|ExecutionSequence`
    (:`then_0`
      (`self.UseMG`))))

(event `InputAction|Attack2`
  (params (Key :type "Key Structure"))
  ;[1 1 1] コメント
  (:`Pressed`
    (bind _success (`self.Is Can Use Weapon` "NewEnumerator1"))
    (if _success
      (`self.AtkActionServer`))))

(event `InputAction|Attack1`
  (params (Key :type "Key Structure"))
  ;[1 1 1] Attack1
  (:`Pressed`
    (`self.TJMAttack1ServerPressed`))
  (:`Released`
    (`self.TJMAttack1ServerReleased`)))

(event `AtkActionServer`
  ;[1 1 1] コメント
  (`self.SetStopVelocty` true)
  (`self.SetAnimationServer` "NewEnumerator7")
  (`self.SetMuzzleCorrectionServer` true)
  (`self.GuidedCheck`)
  (goto _label :!via `Reset`))

(event `TJMAttack1ServerPressed`
  ;[1 1 1] Attack1
  (bind _success (`self.Is Can Use Weapon` "NewEnumerator0"))
  (if _success
    (set `self.IsUseMG` true)
    (`self.SetActorHiddenInGame` (`self.MGFunnel`) false)))

(event `TJMAttack2Server`
  ;[1 1 1] コメント
  (`/Engine/EditorBlueprintResources/StandardMacros.DoOnce` false :!label _label
    (:`Completed`
      (`self.LostAmmo` "NewEnumerator1")
      (`self.InflictWeaponCoolTime` "NewEnumerator1")
      (`self.Attack2Shot`))))

(event `TJMAttack1ServerReleased`
  ;[1 1 1] Attack1
  (set `self.IsUseMG` false)
  (`self.SetActorHiddenInGame` (`self.MGFunnel`) true))

(event `InputAction|Special1`
  (params (Key :type "Key Structure"))
  ;[1 1 1] Special1
  (:`Pressed`
    (bind _success (`self.Is Can Use Weapon` "NewEnumerator2"))
    (if _success
      (`self.TJMSpecial1Server`))))

(event `InputAction|Special2`
  (params (Key :type "Key Structure"))
  ;[1 1 1] Special2
  (:`Pressed`
    (bind _success (`self.Is Can Use Weapon` "NewEnumerator3"))
    (if _success
      (`self.Sp2ActionServer`))))

(event `TJMSpecial1Server`
  ;[1 1 1] Special1
  (`self.LostAmmo` "NewEnumerator2")
  (`self.InflictWeaponCoolTime` "NewEnumerator2")
  (`self.UnfoldingFunnel`)
  (`KismetSystemLibrary.Delay` 4.0)
  (`self.UnunfoldingFunnel`)
  (`self.ReloadAttack2`))

(event `Sp2ActionServer`
  ;[1 1 1] Special2
  (`self.SetStopVelocty` true)
  (`self.SetAnimationServer` "NewEnumerator8")
  (`self.SetMuzzleCorrectionServer` true)
  (goto _label_2 :!via `Reset`))

(event `TJMSpecial2Server`
  ;[1 1 1] Special2
  (`/Engine/EditorBlueprintResources/StandardMacros.DoOnce` false :!label _label_2
    (:`Completed`
      (`self.LostAmmo` "NewEnumerator3")
      (`self.InflictWeaponCoolTime` "NewEnumerator3")
      (`self.TJMSp2Shot`))))

(fn `Attack2Shot`
  (bind _funnel_lf (`self.Funnel_LF`))
  (bind _funnel_rb (`self.Funnel_RB`))
  (bind _funnel_lb (`self.Funnel_LB`))
  (bind _funnel_rf (`self.Funnel_RF`))
  (bind _returnvalue (`KismetMathLibrary.FindLookAtRotation` (`self.K2_GetActorLocation` _funnel_lf) (`self.K2_GetActorLocation` (`self.Target`))))
  (bind _returnvalue_2 (`KismetMathLibrary.FindLookAtRotation` (`self.K2_GetActorLocation` _funnel_rf) (`self.K2_GetActorLocation` (`self.Target`))))
  (bind _returnvalue_3 (`KismetMathLibrary.FindLookAtRotation` (`self.K2_GetActorLocation` _funnel_rb) (`self.K2_GetActorLocation` (`self.Target`))))
  (bind _returnvalue_4 (`KismetMathLibrary.FindLookAtRotation` (`self.K2_GetActorLocation` _funnel_lb) (`self.K2_GetActorLocation` (`self.Target`))))
  (if (`/Game/GameAssets/BluePrint/Bullets/Funnel/BP_Funnel.IsAttach` _funnel_rf)
    (`self.SetGuidance` _funnel_rf)
    (set `/Game/GameAssets/BluePrint/Bullets/Funnel/BP_Funnel.IsAttach` false _funnel_rf)
    (`PrimitiveComponent.SetCollisionEnabled` (`/Game/GameAssets/BluePrint/Bullets/BP_BuletBase.DamageCapsule` _funnel_rf) "QueryOnly")
    (set `/Game/GameAssets/BluePrint/Bullets/BP_BuletBase.Target` (`self.Target`) _funnel_rf)
    (set `/Game/GameAssets/BluePrint/Bullets/BP_BuletBase.MoveDirection` (`KismetMathLibrary.GetForwardVector` _returnvalue_2) _funnel_rf)
    (set `/Game/GameAssets/BluePrint/Bullets/BP_BuletBase.MoveRotation` _returnvalue_2 _funnel_rf)
    (bind _weaponstatus (`self.GetWeaponStatus` "NewEnumerator1"))
    (bind _damagestatus (`self.GetDamageStatus` _weaponstatus))
    (set `/Game/GameAssets/BluePrint/Bullets/BP_BuletBase.DamageStruct` _damagestatus _funnel_rf)
    (set `/Game/GameAssets/BluePrint/Bullets/BP_BuletBase.ShotPosition` (`self.K2_GetActorLocation`) _funnel_rf)
    (`self.FireSeting` _funnel_rf)
    (elif (`/Game/GameAssets/BluePrint/Bullets/Funnel/BP_Funnel.IsAttach` _funnel_lf)
      (`self.SetGuidance` _funnel_lf)
      (set `/Game/GameAssets/BluePrint/Bullets/Funnel/BP_Funnel.IsAttach` false _funnel_lf)
      (`PrimitiveComponent.SetCollisionEnabled` (`/Game/GameAssets/BluePrint/Bullets/BP_BuletBase.DamageCapsule` _funnel_lf) "QueryOnly")
      (set `/Game/GameAssets/BluePrint/Bullets/BP_BuletBase.Target` (`self.Target`) _funnel_lf)
      (set `/Game/GameAssets/BluePrint/Bullets/BP_BuletBase.MoveDirection` (`KismetMathLibrary.GetForwardVector` _returnvalue) _funnel_lf)
      (set `/Game/GameAssets/BluePrint/Bullets/BP_BuletBase.MoveRotation` _returnvalue _funnel_lf)
      (bind _weaponstatus_2 (`self.GetWeaponStatus` "NewEnumerator1"))
      (bind _damagestatus_2 (`self.GetDamageStatus` _weaponstatus_2))
      (set `/Game/GameAssets/BluePrint/Bullets/BP_BuletBase.DamageStruct` _damagestatus_2 _funnel_lf)
      (set `/Game/GameAssets/BluePrint/Bullets/BP_BuletBase.ShotPosition` (`self.K2_GetActorLocation`) _funnel_lf)
      (`self.FireSeting` _funnel_lf)
      (elif (`/Game/GameAssets/BluePrint/Bullets/Funnel/BP_Funnel.IsAttach` _funnel_rb)
        (`self.SetGuidance` _funnel_rb)
        (set `/Game/GameAssets/BluePrint/Bullets/Funnel/BP_Funnel.IsAttach` false _funnel_rb)
        (`PrimitiveComponent.SetCollisionEnabled` (`/Game/GameAssets/BluePrint/Bullets/BP_BuletBase.DamageCapsule` _funnel_rb) "QueryOnly")
        (set `/Game/GameAssets/BluePrint/Bullets/BP_BuletBase.Target` (`self.Target`) _funnel_rb)
        (set `/Game/GameAssets/BluePrint/Bullets/BP_BuletBase.MoveDirection` (`KismetMathLibrary.GetForwardVector` _returnvalue_3) _funnel_rb)
        (set `/Game/GameAssets/BluePrint/Bullets/BP_BuletBase.MoveRotation` _returnvalue_3 _funnel_rb)
        (bind _weaponstatus_3 (`self.GetWeaponStatus` "NewEnumerator1"))
        (bind _damagestatus_3 (`self.GetDamageStatus` _weaponstatus_3))
        (set `/Game/GameAssets/BluePrint/Bullets/BP_BuletBase.DamageStruct` _damagestatus_3 _funnel_rb)
        (set `/Game/GameAssets/BluePrint/Bullets/BP_BuletBase.ShotPosition` (`self.K2_GetActorLocation`) _funnel_rb)
        (`self.FireSeting` _funnel_rb)
        (elif (`/Game/GameAssets/BluePrint/Bullets/Funnel/BP_Funnel.IsAttach` _funnel_lb)
          (`self.SetGuidance` _funnel_lb)
          (set `/Game/GameAssets/BluePrint/Bullets/Funnel/BP_Funnel.IsAttach` false _funnel_lb)
          (`PrimitiveComponent.SetCollisionEnabled` (`/Game/GameAssets/BluePrint/Bullets/BP_BuletBase.DamageCapsule` _funnel_lb) "QueryOnly")
          (set `/Game/GameAssets/BluePrint/Bullets/BP_BuletBase.Target` (`self.Target`) _funnel_lb)
          (set `/Game/GameAssets/BluePrint/Bullets/BP_BuletBase.MoveDirection` (`KismetMathLibrary.GetForwardVector` _returnvalue_4) _funnel_lb)
          (set `/Game/GameAssets/BluePrint/Bullets/BP_BuletBase.MoveRotation` _returnvalue_4 _funnel_lb)
          (bind _weaponstatus_4 (`self.GetWeaponStatus` "NewEnumerator1"))
          (bind _damagestatus_4 (`self.GetDamageStatus` _weaponstatus_4))
          (set `/Game/GameAssets/BluePrint/Bullets/BP_BuletBase.DamageStruct` _damagestatus_4 _funnel_lb)
          (set `/Game/GameAssets/BluePrint/Bullets/BP_BuletBase.ShotPosition` (`self.K2_GetActorLocation`) _funnel_lb)
          (`self.FireSeting` _funnel_lb))))))

(fn `Damage HP`
  (params (Damage :type "Float (double-precision)") (MinDamage :type "Float (double-precision)") (Attacker :type "/Game/GameAssets/BluePrint/Characters/BP_CharacterBase Object Reference"))
  (returns (AeakenWithstand :type Boolean) (Dead :type Boolean))
  (bind _funnel_rf (`self.Funnel_RF`))
  (bind _funnel_rb (`self.Funnel_RB`))
  (bind _funnel_lf (`self.Funnel_LF`))
  (bind _funnel_lb (`self.Funnel_LB`))
  (bind (_aeakenwithstand _dead) (`parent.Damage HP` Damage MinDamage Attacker))
  (if _dead
    (`self.SetActorHiddenInGame` _funnel_rf true)
    (`self.SetActorHiddenInGame` _funnel_rb true)
    (`self.SetActorHiddenInGame` _funnel_lf true)
    (`self.SetActorHiddenInGame` _funnel_lb true)
    (`self.SetActorHiddenInGame` (`self.MGFunnel`) true)
    (set `/Game/GameAssets/BluePrint/Bullets/Funnel/BP_Funnel.IsAttach` true _funnel_rf)
    (set `/Game/GameAssets/BluePrint/Bullets/Funnel/BP_Funnel.IsAttach` true _funnel_rb)
    (set `/Game/GameAssets/BluePrint/Bullets/Funnel/BP_Funnel.IsAttach` true _funnel_lf)
    (set `/Game/GameAssets/BluePrint/Bullets/Funnel/BP_Funnel.IsAttach` true _funnel_lb)
    (return _aeakenwithstand true)
    (else
      (return _aeakenwithstand false))))

(fn `FunnelSpawn`
  (locals (RFName :type Name :default "funnel_socket_rf") (RBName :type Name :default "funnel_socket_rb") (LFName :type Name :default "funnel_socket_lf") (LBName :type Name :default "funnel_socket_lb") (MGName :type Name :default "funnel_socket_mg"))
  (bind _rfname (`local.RFName`))
  (bind _rbname (`local.RBName`))
  (bind _lfname (`local.LFName`))
  (bind _lbname (`local.LBName`))
  (bind _mgname (`local.MGName`))
  (`|ExecutionSequence`
    (:`then_0`
      (if (== (`self.Funnel_RF`) null)
        (bind _returnvalue (`|SpawnActorFromClass` "/Game/GameAssets/BluePrint/Bullets/Funnel/TJM/BP_Funnel_TJM.BP_Funnel_TJM_C" (`KismetMathLibrary.Conv_VectorToTransform` (`SceneComponent.GetSocketLocation` (`self.Mesh`) _rfname)) "Undefined" "OverrideRootScale" null null))
        (set `/Game/GameAssets/BluePrint/Bullets/Funnel/BP_Funnel.Master` self _returnvalue)
        (set `self.Funnel_RF` _returnvalue)
        (set `/Game/GameAssets/BluePrint/Bullets/Funnel/BP_Funnel.AttachSocketName` _rfname _returnvalue)
        (set `/Game/GameAssets/BluePrint/Bullets/Funnel/TJM/BP_Funnel_TJM.PositionName` "NewEnumerator0" _returnvalue)))
    (:`then_1`
      (if (== (`self.Funnel_RB`) null)
        (bind _returnvalue_2 (`|SpawnActorFromClass` "/Game/GameAssets/BluePrint/Bullets/Funnel/TJM/BP_Funnel_TJM.BP_Funnel_TJM_C" (`KismetMathLibrary.Conv_VectorToTransform` (`SceneComponent.GetSocketLocation` (`self.Mesh`) _rbname)) "Undefined" "OverrideRootScale" null null))
        (set `/Game/GameAssets/BluePrint/Bullets/Funnel/BP_Funnel.Master` self _returnvalue_2)
        (set `self.Funnel_RB` _returnvalue_2)
        (set `/Game/GameAssets/BluePrint/Bullets/Funnel/BP_Funnel.AttachSocketName` _rbname _returnvalue_2)
        (set `/Game/GameAssets/BluePrint/Bullets/Funnel/TJM/BP_Funnel_TJM.PositionName` "NewEnumerator1" _returnvalue_2)))
    (:`then_2`
      (if (== (`self.Funnel_LF`) null)
        (bind _returnvalue_3 (`|SpawnActorFromClass` "/Game/GameAssets/BluePrint/Bullets/Funnel/TJM/BP_Funnel_TJM.BP_Funnel_TJM_C" (`KismetMathLibrary.Conv_VectorToTransform` (`SceneComponent.GetSocketLocation` (`self.Mesh`) _lfname)) "Undefined" "OverrideRootScale" null null))
        (set `/Game/GameAssets/BluePrint/Bullets/Funnel/BP_Funnel.Master` self _returnvalue_3)
        (set `self.Funnel_LF` _returnvalue_3)
        (set `/Game/GameAssets/BluePrint/Bullets/Funnel/BP_Funnel.AttachSocketName` _lfname _returnvalue_3)
        (set `/Game/GameAssets/BluePrint/Bullets/Funnel/TJM/BP_Funnel_TJM.PositionName` "NewEnumerator2" _returnvalue_3)))
    (:`then_3`
      (if (== (`self.Funnel_LB`) null)
        (bind _returnvalue_4 (`|SpawnActorFromClass` "/Game/GameAssets/BluePrint/Bullets/Funnel/TJM/BP_Funnel_TJM.BP_Funnel_TJM_C" (`KismetMathLibrary.Conv_VectorToTransform` (`SceneComponent.GetSocketLocation` (`self.Mesh`) _lbname)) "Undefined" "OverrideRootScale" null null))
        (set `/Game/GameAssets/BluePrint/Bullets/Funnel/BP_Funnel.Master` self _returnvalue_4)
        (set `self.Funnel_LB` _returnvalue_4)
        (set `/Game/GameAssets/BluePrint/Bullets/Funnel/BP_Funnel.AttachSocketName` _lbname _returnvalue_4)
        (set `/Game/GameAssets/BluePrint/Bullets/Funnel/TJM/BP_Funnel_TJM.PositionName` "NewEnumerator3" _returnvalue_4)))
    (:`then_4`
      (if (== (`self.MGFunnel`) null)
        (bind _returnvalue_5 (`|SpawnActorFromClass` "/Game/GameAssets/BluePrint/Bullets/Funnel/TJM/BP_MGFunnel_TJM.BP_MGFunnel_TJM_C" (`KismetMathLibrary.Conv_VectorToTransform` (`SceneComponent.GetSocketLocation` (`self.Mesh`) _mgname)) "Undefined" "OverrideRootScale" null null))
        (set `/Game/GameAssets/BluePrint/Bullets/Funnel/BP_Funnel.Master` self _returnvalue_5)
        (set `self.MGFunnel` _returnvalue_5)
        (set `/Game/GameAssets/BluePrint/Bullets/Funnel/BP_Funnel.AttachSocketName` _mgname _returnvalue_5)))))

(fn `ReloadAttack2`
  (bind (_weaponstatus _number) (`self.GetWeaponStatus` "NewEnumerator1"))
  (bind _structout (setmembers `/Game/GameAssets/BluePrint/Struct/STRUCT_Weapon` :`StructRef` _weaponstatus :`NowAmmo` (`.MaxAmmo_2_A5CCF65F4F6A778A6C75B08A3A5FE964` (break `/Game/GameAssets/BluePrint/Struct/STRUCT_Weapon` _weaponstatus))))
  (`KismetArrayLibrary.Array_Set` (`self.WeaponStatus`) _number _structout))

(fn `RespawnProcessing`
  (bind _returnvalue (`self.K2_GetActorRotation`))
  (bind _returnvalue_2 (`self.K2_GetActorRotation`))
  (bind _mesh (`self.Mesh`))
  (bind _funnel_rb (`self.Funnel_RB`))
  (bind _funnel_lb (`self.Funnel_LB`))
  (bind _funnel_lf (`self.Funnel_LF`))
  (bind _mesh_2 (`self.Mesh`))
  (bind _funnel_rf (`self.Funnel_RF`))
  (`parent.RespawnProcessing`)
  (`|ExecutionSequence`
    (:`then_0`
      (`/Engine/EditorBlueprintResources/StandardMacros.IsValid` _funnel_rf
        (:`Is Valid`
          (`self.SetActorHiddenInGame` _funnel_rf false)
          (`self.K2_SetActorLocation` _funnel_rf (`SceneComponent.GetSocketLocation` _mesh_2 (`/Game/GameAssets/BluePrint/Bullets/Funnel/BP_Funnel.AttachSocketName` _funnel_rf)) false true)
          (`self.K2_SetActorRotation` _funnel_rf _returnvalue false))))
    (:`then_1`
      (`/Engine/EditorBlueprintResources/StandardMacros.IsValid` _funnel_rb
        (:`Is Valid`
          (`self.SetActorHiddenInGame` _funnel_rb false)
          (`self.K2_SetActorLocation` _funnel_rb (`SceneComponent.GetSocketLocation` _mesh_2 (`/Game/GameAssets/BluePrint/Bullets/Funnel/BP_Funnel.AttachSocketName` _funnel_rb)) false true)
          (`self.K2_SetActorRotation` _funnel_rb _returnvalue false))))
    (:`then_2`
      (`/Engine/EditorBlueprintResources/StandardMacros.IsValid` _funnel_lf
        (:`Is Valid`
          (`self.SetActorHiddenInGame` _funnel_lf false)
          (`self.K2_SetActorLocation` _funnel_lf (`SceneComponent.GetSocketLocation` _mesh (`/Game/GameAssets/BluePrint/Bullets/Funnel/BP_Funnel.AttachSocketName` _funnel_lf)) false true)
          (`self.K2_SetActorRotation` _funnel_lf _returnvalue_2 false))))
    (:`then_3`
      (`/Engine/EditorBlueprintResources/StandardMacros.IsValid` _funnel_lb
        (:`Is Valid`
          (`self.SetActorHiddenInGame` _funnel_lb false)
          (`self.K2_SetActorLocation` _funnel_lb (`SceneComponent.GetSocketLocation` _mesh (`/Game/GameAssets/BluePrint/Bullets/Funnel/BP_Funnel.AttachSocketName` _funnel_lb)) false true)
          (`self.K2_SetActorRotation` _funnel_lb _returnvalue_2 false))))))

(fn `SearchShotPosition`
  (returns (ShotTransform :type "Transform Structure"))
  (bind _mgfunnel (`self.MGFunnel`))
  (set `/Game/GameAssets/BluePrint/Bullets/BP_BuletBase.Target` (`self.Target`) _mgfunnel)
  (return (`KismetMathLibrary.Conv_VectorToTransform` (`SceneComponent.K2_GetComponentLocation` (`/Game/GameAssets/BluePrint/Bullets/Funnel/TJM/BP_MGFunnel_TJM.ShotPoint` _mgfunnel)))))

(fn `TJMAtk1Bulet`
  (params (SpawnTransform :type "Transform Structure"))
  (bind _target (`self.Target`))
  (bind _returnvalue (`self.GetActorForwardVector` (`GameplayStatics.GetPlayerController` 0)))
  (bind _returnvalue_2 (`|SpawnActorFromClass` "/Game/GameAssets/BluePrint/Bullets/Beam/BP_test_beam.BP_test_beam_C" SpawnTransform "Undefined" "OverrideRootScale" null null))
  ;[1 0.4983 0.5381] コメント
  (`self.FireSeting` _returnvalue_2)
  (`|ExecutionSequence`
    (:`then_0`
      (`/Game/GameAssets/BluePrint/Method/BP_MacroLibrary.IsTargetExistence` _target
        (:`NotExistence`
          (`self.K2_SetActorRotation` _returnvalue_2 (`self.K2_GetActorRotation`) false))
        (:`Existence`
          (bind _returnvalue_3 (`KismetMathLibrary.FindLookAtRotation` (`self.K2_GetActorLocation` _returnvalue_2) (`self.K2_GetActorLocation` (`self.Target`))))
          (`self.K2_SetActorRotation` _returnvalue_2 _returnvalue_3 false)
          (set `/Game/GameAssets/BluePrint/Bullets/BP_BuletBase.MoveDirection` _returnvalue _returnvalue_2)
          (set `/Game/GameAssets/BluePrint/Bullets/BP_BuletBase.Target` (`self.Target`) _returnvalue_2))))
    (:`then_1`
      (`/Game/GameAssets/BluePrint/Method/BP_MacroLibrary.IsTargetExistence` _target
        (:`NotExistence`
          (set `/Game/GameAssets/BluePrint/Bullets/BP_BuletBase.MoveRotation` (`self.K2_GetActorRotation`) _returnvalue_2)
          (set `/Game/GameAssets/BluePrint/Bullets/BP_BuletBase.MoveDirection` _returnvalue _returnvalue_2))
        (:`Existence`
          (set `/Game/GameAssets/BluePrint/Bullets/BP_BuletBase.MoveRotation` _returnvalue_3 _returnvalue_2)
          (set `/Game/GameAssets/BluePrint/Bullets/BP_BuletBase.MoveDirection` (`KismetMathLibrary.GetForwardVector` _returnvalue_3) _returnvalue_2))))
    (:`then_2`
      (`self.SetDamageProcess` _returnvalue_2))))

(fn `TJMSp1Bulet`
  (params (SpawnTransform :type "Transform Structure"))
  (bind _target (`self.Target`))
  (bind _returnvalue (`|SpawnActorFromClass` "/Game/GameAssets/BluePrint/Bullets/Beam/BP_test_beam.BP_test_beam_C" SpawnTransform "Undefined" "OverrideRootScale" null null))
  (`self.FireSeting` _returnvalue)
  (`|ExecutionSequence`
    (:`then_0`
      (`/Game/GameAssets/BluePrint/Method/BP_MacroLibrary.IsTargetExistence` _target
        (:`NotExistence`
          (`self.K2_SetActorRotation` _returnvalue (`self.K2_GetActorRotation`) false))
        (:`Existence`
          (bind _returnvalue_2 (`KismetMathLibrary.FindLookAtRotation` (`self.K2_GetActorLocation` _returnvalue) (`self.K2_GetActorLocation` (`self.Target`))))
          (`self.K2_SetActorRotation` _returnvalue _returnvalue_2 false)
          (set `/Game/GameAssets/BluePrint/Bullets/BP_BuletBase.Target` (`self.Target`) _returnvalue))))
    (:`then_1`
      (`/Game/GameAssets/BluePrint/Method/BP_MacroLibrary.IsTargetExistence` _target
        (:`NotExistence`
          (set `/Game/GameAssets/BluePrint/Bullets/BP_BuletBase.MoveRotation` (`self.K2_GetActorRotation`) _returnvalue)
          (set `/Game/GameAssets/BluePrint/Bullets/BP_BuletBase.MoveDirection` (`self.GetActorForwardVector` (`GameplayStatics.GetPlayerController` 0)) _returnvalue))
        (:`Existence`
          (set `/Game/GameAssets/BluePrint/Bullets/BP_BuletBase.MoveRotation` _returnvalue_2 _returnvalue)
          (set `/Game/GameAssets/BluePrint/Bullets/BP_BuletBase.MoveDirection` (`KismetMathLibrary.GetForwardVector` _returnvalue_2) _returnvalue))))
    (:`then_2`
      (`self.SetDamageProcess` _returnvalue "NewEnumerator2"))))

(fn `TJMSp2Shot`
  (bind _target (`self.Target`))
  (bind _returnvalue (`self.GetActorForwardVector` (`GameplayStatics.GetPlayerController` 0)))
  (bind _returnvalue_2 (`|SpawnActorFromClass` "/Game/GameAssets/BluePrint/Bullets/GeroBeam/BP_GeroBeam_TJM.BP_GeroBeam_TJM_C" (`SceneComponent.K2_GetComponentToWorld` (`self.GeroBeamPoint`)) "Undefined" "OverrideRootScale" null null))
  (set `/Game/GameAssets/BluePrint/Bullets/BP_BuletBase.FlightTime` 4.0 _returnvalue_2)
  (`self.FireSeting` _returnvalue_2)
  (`|ExecutionSequence`
    (:`then_0`
      (`/Game/GameAssets/BluePrint/Method/BP_MacroLibrary.IsTargetExistence` _target
        (:`NotExistence`
          (`self.K2_SetActorRotation` _returnvalue_2 (`self.K2_GetActorRotation`) false))
        (:`Existence`
          (bind _returnvalue_3 (`KismetMathLibrary.FindLookAtRotation` (`self.K2_GetActorLocation` _returnvalue_2) (`self.K2_GetActorLocation` (`self.Target`))))
          (`self.K2_SetActorRotation` _returnvalue_2 _returnvalue_3 false)
          (set `/Game/GameAssets/BluePrint/Bullets/BP_BuletBase.MoveDirection` _returnvalue _returnvalue_2)
          (set `/Game/GameAssets/BluePrint/Bullets/BP_BuletBase.Target` (`self.Target`) _returnvalue_2))))
    (:`then_1`
      (`/Game/GameAssets/BluePrint/Method/BP_MacroLibrary.IsTargetExistence` _target
        (:`NotExistence`
          (set `/Game/GameAssets/BluePrint/Bullets/BP_BuletBase.MoveRotation` (`self.K2_GetActorRotation`) _returnvalue_2)
          (set `/Game/GameAssets/BluePrint/Bullets/BP_BuletBase.MoveDirection` _returnvalue _returnvalue_2))
        (:`Existence`
          (set `/Game/GameAssets/BluePrint/Bullets/BP_BuletBase.MoveRotation` _returnvalue_3 _returnvalue_2)
          (set `/Game/GameAssets/BluePrint/Bullets/BP_BuletBase.MoveDirection` (`KismetMathLibrary.GetForwardVector` _returnvalue_3) _returnvalue_2))))
    (:`then_2`
      (`self.SetDamageProcess` _returnvalue_2 "NewEnumerator3"))))

(fn `UnfoldingFunnel`
  (locals (FireLag :type "Float (double-precision)" :default 0.2))
  (bind _funnel_rf (`self.Funnel_RF`))
  (bind _funnel_rb (`self.Funnel_RB`))
  (bind _funnel_lb (`self.Funnel_LB`))
  (bind _funnel_lf (`self.Funnel_LF`))
  (bind _weaponstatus (`self.GetWeaponStatus` "NewEnumerator2"))
  (bind _damagestatus (`self.GetDamageStatus` _weaponstatus))
  (bind _correctiondamage (`self.DamageCorrection` _damagestatus))
  (`|ExecutionSequence`
    (:`then_0`
      (set `/Game/GameAssets/BluePrint/Bullets/Funnel/TJM/BP_Funnel_TJM.IsUnfolding` true _funnel_rf)
      (set `/Game/GameAssets/BluePrint/Bullets/BP_BuletBase.Target` (`self.Target`) _funnel_rf)
      (set `/Game/GameAssets/BluePrint/Bullets/Funnel/TJM/BP_Funnel_TJM.BeamDamage` _correctiondamage _funnel_rf)
      (bind _output_get (set `/Game/GameAssets/BluePrint/Bullets/Funnel/TJM/BP_Funnel_TJM.FireTimer` 1.5 _funnel_rf))
      (set `/Game/GameAssets/BluePrint/Bullets/Funnel/TJM/BP_Funnel_TJM.Fire` true _funnel_rf))
    (:`then_1`
      (set `/Game/GameAssets/BluePrint/Bullets/Funnel/TJM/BP_Funnel_TJM.IsUnfolding` true _funnel_rb)
      (set `/Game/GameAssets/BluePrint/Bullets/BP_BuletBase.Target` (`self.Target`) _funnel_rb)
      (set `/Game/GameAssets/BluePrint/Bullets/Funnel/TJM/BP_Funnel_TJM.BeamDamage` _correctiondamage _funnel_rb)
      (bind _output_get_2 (set `/Game/GameAssets/BluePrint/Bullets/Funnel/TJM/BP_Funnel_TJM.FireTimer` (+ _output_get (`local.FireLag`)) _funnel_rb))
      (set `/Game/GameAssets/BluePrint/Bullets/Funnel/TJM/BP_Funnel_TJM.Fire` true _funnel_rb))
    (:`then_2`
      (set `/Game/GameAssets/BluePrint/Bullets/Funnel/TJM/BP_Funnel_TJM.IsUnfolding` true _funnel_lf)
      (set `/Game/GameAssets/BluePrint/Bullets/BP_BuletBase.Target` (`self.Target`) _funnel_lf)
      (set `/Game/GameAssets/BluePrint/Bullets/Funnel/TJM/BP_Funnel_TJM.BeamDamage` _correctiondamage _funnel_lf)
      (bind _output_get_3 (set `/Game/GameAssets/BluePrint/Bullets/Funnel/TJM/BP_Funnel_TJM.FireTimer` (+ _output_get_2 (`local.FireLag`)) _funnel_lf))
      (set `/Game/GameAssets/BluePrint/Bullets/Funnel/TJM/BP_Funnel_TJM.Fire` true _funnel_lf))
    (:`then_3`
      (set `/Game/GameAssets/BluePrint/Bullets/Funnel/TJM/BP_Funnel_TJM.IsUnfolding` true _funnel_lb)
      (set `/Game/GameAssets/BluePrint/Bullets/BP_BuletBase.Target` (`self.Target`) _funnel_lb)
      (set `/Game/GameAssets/BluePrint/Bullets/Funnel/TJM/BP_Funnel_TJM.BeamDamage` _correctiondamage _funnel_lb)
      (set `/Game/GameAssets/BluePrint/Bullets/Funnel/TJM/BP_Funnel_TJM.FireTimer` (+ _output_get_3 (`local.FireLag`)) _funnel_lb)
      (set `/Game/GameAssets/BluePrint/Bullets/Funnel/TJM/BP_Funnel_TJM.Fire` true _funnel_lb))))

(fn `UnunfoldingFunnel`
  (bind _funnel_rf (`self.Funnel_RF`))
  (bind _funnel_rb (`self.Funnel_RB`))
  (bind _funnel_lb (`self.Funnel_LB`))
  (bind _funnel_lf (`self.Funnel_LF`))
  (`|ExecutionSequence`
    (:`then_0`
      (set `/Game/GameAssets/BluePrint/Bullets/Funnel/TJM/BP_Funnel_TJM.IsUnfolding` false _funnel_rf)
      (set `/Game/GameAssets/BluePrint/Bullets/Funnel/BP_Funnel.IsAttach` true _funnel_rf)
      (set `/Game/GameAssets/BluePrint/Bullets/Funnel/BP_Funnel.Return` false _funnel_rf))
    (:`then_1`
      (set `/Game/GameAssets/BluePrint/Bullets/Funnel/TJM/BP_Funnel_TJM.IsUnfolding` false _funnel_rb)
      (set `/Game/GameAssets/BluePrint/Bullets/Funnel/BP_Funnel.IsAttach` true _funnel_rb)
      (set `/Game/GameAssets/BluePrint/Bullets/Funnel/BP_Funnel.Return` false _funnel_rb))
    (:`then_2`
      (set `/Game/GameAssets/BluePrint/Bullets/Funnel/TJM/BP_Funnel_TJM.IsUnfolding` false _funnel_lf)
      (set `/Game/GameAssets/BluePrint/Bullets/Funnel/BP_Funnel.IsAttach` true _funnel_lf)
      (set `/Game/GameAssets/BluePrint/Bullets/Funnel/BP_Funnel.Return` false _funnel_lf))
    (:`then_3`
      (set `/Game/GameAssets/BluePrint/Bullets/Funnel/TJM/BP_Funnel_TJM.IsUnfolding` false _funnel_lb)
      (set `/Game/GameAssets/BluePrint/Bullets/Funnel/BP_Funnel.IsAttach` true _funnel_lb)
      (set `/Game/GameAssets/BluePrint/Bullets/Funnel/BP_Funnel.Return` false _funnel_lb))))

(fn `UseMG`
  (if (`self.IsUseMG`)
    (`self.GuidedCheck`)
    (bind _success (`self.Is Can Use Weapon` "NewEnumerator0"))
    (if _success
      (`self.UseMGServer`))))

(fn `UserConstructionScript`
  (`parent.UserConstructionScript`))