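; Beam projectile that stays in place, extends its damage capsule up to a max length, and destroys itself when its flight time runs out.
; Tick enables the capsule's query collision for one frame per hit interval, so overlaps re-fire as periodic hits.
; HitCheck filters by ConsortPlaneValue: box hits trigger guard and record the character in GuardActor, while tagged HitCapsule hits damage characters not recorded there.
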(event `self.ReceiveBeginPlay`
  (set `MovementComponent.Velocity` (0.0 0.0 0.0) (`self.ProjectileMovement`))
  (`PrimitiveComponent.SetCollisionEnabled` (`self.DamageCapsule`) "NoCollision"))

(event `self.ReceiveTick`
  (params (DeltaSeconds :type "Float (single-precision)"))
  (bind _damagecapsule2 (`self.DamageCapsule2`))
  (bind _damagecapsule2_2 (`self.DamageCapsule2`))
  (bind _returnvalue (`KismetMathLibrary.FClamp` (+ (`CapsuleComponent.CapsuleHalfHeight` _damagecapsule2) (* DeltaSeconds (`self.BeSmoothedSpeed`))) 0.0 (`self.MaxLength`)))
  (`|ExecutionSequence`
    (:`then_0`
      (`CapsuleComponent.SetCapsuleHalfHeight` _damagecapsule2 _returnvalue true)
      (`SceneComponent.K2_SetRelativeLocation` _damagecapsule2 (`KismetMathLibrary.MakeVector` 0.0 0.0 _returnvalue) false false))
    (:`then_1`
      (if (<= (`self.HitIntervalTimer`) 0.0)
        (set `self.HitIntervalTimer` (`self.HitInterval`))
        (`PrimitiveComponent.SetCollisionEnabled` _damagecapsule2_2 "QueryOnly")
        (else
          (set `self.HitIntervalTimer` (- (`self.HitIntervalTimer`) DeltaSeconds))
          (`PrimitiveComponent.SetCollisionEnabled` _damagecapsule2_2 "NoCollision"))))
    (:`then_2`
      (`self.FlightTimeProcess`)
      (if (<= (`self.FlightTime`) 0.0)
        (`self.K2_DestroyActor`)))))

(event `self.DamageCapsule2.OnComponentBeginOverlap`
  (params (OverlappedComponent :type "PrimitiveComponent Object Reference") (OtherActor :type "Actor Object Reference") (OtherComp :type "PrimitiveComponent Object Reference") (OtherBodyIndex :type Integer) (bFromSweep :type Boolean) (SweepResult :type "HitResult Structure (by ref)"))
  ;[1 1 1] 当たり判定処理
  (`self.HitCheck` OtherActor OtherComp))

(fn `HitCheck`
  (params (Actor :type "Object Object Reference") (Component :type "Object Object Reference"))
  (bind _guardactor (`self.GuardActor`))
  (if (!= (`self.ConsortPlaneValue`) -1)
    (bind _asbp_character_base (cast `/Game/GameAssets/BluePrint/Characters/BP_CharacterBase` Actor))
    (if (!= (`self.ConsortPlaneValue`) (`/Game/GameAssets/BluePrint/Characters/BP_CharacterBase.ConsortPlaneValue` _asbp_character_base))
      (cast `BoxComponent` Component
        (:`then`
          (`/Game/GameAssets/BluePrint/Characters/BP_CharacterBase.SetGuardServer` _asbp_character_base 1.0)
          (if (not (`KismetArrayLibrary.Array_Contains` _guardactor _asbp_character_base))
            (`KismetArrayLibrary.Array_Add` _guardactor _asbp_character_base)))
        (:`CastFailed`
          (if (not (`KismetArrayLibrary.Array_Contains` _guardactor _asbp_character_base))
            (bind _ascapsule_collision (cast `CapsuleComponent` Component))
            (for _array_element (`ActorComponent.ComponentTags` _ascapsule_collision)
              (if (== _array_element "HitCapsule")
                (bind _asbp_character_base_2 (cast `/Game/GameAssets/BluePrint/Characters/BP_CharacterBase` Actor))
                (if (!= (`self.ConsortPlaneValue`) (`/Game/GameAssets/BluePrint/Characters/BP_CharacterBase.ConsortPlaneValue` _asbp_character_base_2))
                  (`self.DamageServer` _asbp_character_base_2))))))))))

(fn `UserConstructionScript`
  (`parent.UserConstructionScript`))