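; MAI's ultimate beam projectile, a homing bullet that loads its movement settings from the "MAI_ULT" status on BeginPlay.
; Each tick it wraps its move rotation to ±180 degrees, destroys itself when its time-based range expires, then steers and moves using shared bullet functions.
; DamageCapsule overlaps run the hit check, while blocking hits on actors tagged BulletBlocker destroy the beam.
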(event `self.ReceiveBeginPlay`
  (`self.SetBulletMoveStatus` "MAI_ULT"))

(event `self.ReceiveTick`
  (params (DeltaSeconds :type "Float (single-precision)"))
  (bind _outrotator (`/Game/GameAssets/BluePrint/Method/test_method.ConversionAngleTo-180_180` (`self.MoveRotation`)))
  (set `self.MoveRotation` _outrotator)
  (`|ExecutionSequence`
    (:`then_0`
      ;[1 1 1] 射程（時間）がきたら消す
      (bind _destroy (`self.FightTImeProcessing` DeltaSeconds))
      (if _destroy
        (`self.K2_DestroyActor`)))
    (:`then_1`
      ;[1 1 1] 誘導する動き（進む方向を変える）
      (`self.ChangeDirectionProcessing`)
      ;[1 1 1] 移動処理
      (`self.Move` DeltaSeconds))))

(event `self.DamageCapsule.OnComponentBeginOverlap`
  (params (OverlappedComponent :type "PrimitiveComponent Object Reference") (OtherActor :type "Actor Object Reference") (OtherComp :type "PrimitiveComponent Object Reference") (OtherBodyIndex :type Integer) (bFromSweep :type Boolean) (SweepResult :type "HitResult Structure (by ref)"))
  ;[1 1 1] Hit判定
  (`self.HitCheck` OtherActor OtherComp))

(event `self.DamageCapsule.OnComponentHit`
  (params (HitComponent :type "PrimitiveComponent Object Reference") (OtherActor :type "Actor Object Reference") (OtherComp :type "PrimitiveComponent Object Reference") (NormalImpulse :type "Vector Structure") (Hit :type "HitResult Structure (by ref)"))
  ;[1 1 1] ブロック判定
  (if (`self.ActorHasTag` OtherActor "BulletBlocker")
    (`self.K2_DestroyActor`)))

(fn `UserConstructionScript`
  (`parent.UserConstructionScript`))