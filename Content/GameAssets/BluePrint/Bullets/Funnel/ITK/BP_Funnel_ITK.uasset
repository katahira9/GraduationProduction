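; Funnel projectile (ITK variant) that trails a socket on its Master's mesh while attached and flies at a Target when detached.
; Tick switches between lerped socket following and free flight, where it homes until the target leaves the guidance angle, then disables damage collision after a short delay.
; When Return is set, it steers back toward the socket.
; DamageCapsule overlaps go to HitCheck, and a custom event sets speed and guidance tuning.
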(event `CustomEvent`
  ;[1 1 1] BeginPlay
  (set `self.MaxSpeed` 2000.0)
  (set `self.GuidedValue_Yaw` 0.5)
  (set `self.GuidedMaxAngle_Pitch` 0.5)
  (set `self.GuidedValue_Pich` 10.0)
  (set `self.GuidedMaxAngle_Yaw` 20.0))

(event `self.ReceiveTick`
  (params (DeltaSeconds :type "Float (single-precision)"))
  ;[1 1 1] Tick
  (`/Engine/EditorBlueprintResources/StandardMacros.IsValid` self
    (:`Is Valid`
      (if (`self.IsAttach`)
        (`self.AttachMove` DeltaSeconds)
        (goto _label :!via `Reset`)
        (else
          (`self.NotAttachMove` DeltaSeconds)
          (`/Engine/EditorBlueprintResources/StandardMacros.DoOnce` false :!label _label
            (:`Completed`
              (`self.LookUp` (`self.K2_GetActorLocation` (`self.Target`))))))))))

(event `self.DamageCapsule.OnComponentBeginOverlap`
  (params (OverlappedComponent :type "PrimitiveComponent Object Reference") (OtherActor :type "Actor Object Reference") (OtherComp :type "PrimitiveComponent Object Reference") (OtherBodyIndex :type Integer) (bFromSweep :type Boolean) (SweepResult :type "HitResult Structure (by ref)"))
  (`self.HitCheck` OtherActor OtherComp))

(fn `AttachMove`
  (params (DeltaTIme :type "Float (double-precision)"))
  (locals (NewLocalVar_0 :type Boolean))
  (`self.K2_AddActorWorldOffset` (`KismetMathLibrary.VLerp` (0.0 0.0 0.0) (- (`SceneComponent.GetSocketLocation` (`Character.Mesh` (`self.Master`)) (`self.AttachSocketName`)) (`self.K2_GetActorLocation`)) 0.2))
  (`self.K2_SetActorRotation` (`self.K2_GetActorRotation` (`self.Master`))))

(fn `GoingToMoveDirection`
  (params (DeltaTime :type "Float (double-precision)") (Speed :type "Float (double-precision)"))
  (`self.K2_AddActorWorldTransform` (`KismetMathLibrary.Conv_VectorToTransform` (* (`self.MoveDirection`) (* DeltaTime Speed)))))

(fn `LookUp`
  (params (Location :type "Vector Structure"))
  (bind (_x _y _z) (`KismetMathLibrary.BreakRotIntoAxes` (`KismetMathLibrary.FindLookAtRotation` (`self.K2_GetActorLocation`) Location)))
  (`self.K2_SetActorRotation` (`KismetMathLibrary.MakeRotationFromAxes` _z _y (* _x -1))))

(fn `NotAttachMove`
  (params (DeltaTime :type "Float (double-precision)"))
  (bind _attachsocketname (`self.AttachSocketName`))
  (bind _mesh (`Character.Mesh` (`self.Master`)))
  (bind _returnvalue (`SceneComponent.GetSocketLocation` _mesh _attachsocketname))
  (bind _returnvalue_2 (- _returnvalue (`self.K2_GetActorLocation`)))
  (if (`self.Return`)
    (if (`SceneComponent.DoesSocketExist` _mesh _attachsocketname)
      (`|ExecutionSequence`
        (:`then_0`
          (set `self.MoveDirection` (`KismetMathLibrary.Normal` (`KismetMathLibrary.VLerp` (`self.MoveDirection`) (`KismetMathLibrary.Normal` _returnvalue_2) 0.25)))
          (set `self.ConsortPlaneValue` -1))
        (:`then_1`
          (`self.GoingToMoveDirection` DeltaTime (`self.ReturnSpeed`))
          (`self.LookUp` _returnvalue)
          (if (< (`KismetMathLibrary.VSize` _returnvalue_2) 20.0)
            (set `self.Return` false)
            (set `self.IsAttach` false)
            (set `self.AftertasteTimer` 0.0)))))
    (else
      (`|ExecutionSequence`
        (:`then_0`
          (`self.GoingToMoveDirection` DeltaTime (`self.MaxSpeed`))
          (if (> (`self.AftertasteTimer`) 0.0)
            _
            (elif (`self.IsGuided`)
              (`self.LookUp` (`self.K2_GetActorLocation` (`self.Target`))))))
        (:`then_1`
          (`self.IsTargetExistence`
            (:`Existence`
              (if (> (`KismetMathLibrary.DegAcos` (`KismetMathLibrary.Dot_VectorVector` (`self.MoveDirection`) (`self.DirectionToTarget`))) (`self.GuidedAngle`))
                (set `self.IsGuided` false)
                (set `self.ShotPosition` (`self.K2_GetActorLocation`))
                (bind _output_get (set `self.AftertasteTimer` (+ (`self.AftertasteTimer`) DeltaTime)))
                (if (>= _output_get 0.3)
                  (set `self.Return` false)
                  (set `self.AftertasteTimer` 0.0)
                  (`PrimitiveComponent.SetCollisionEnabled` (`self.DamageCapsule`) "NoCollision"))
                (else
                  (`self.ChangeDirectionProcessing`))))))))))

(fn `UserConstructionScript`)