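; Funnel drone for ta-jimaharu that follows its master, fires beams and flies as a homing projectile.
; Tick selects attached, detached or ultimate movement, lerping toward a socket or, when unfolded, a target-relative formation slot.
; Unfolded funnels face the target and trigger the master's beam shot on a timer.
; Flight steers until the target stays outside the guidance angle briefly, then disables damage collision and flags return, or reattaches after an ultimate.
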(event `self.ReceiveBeginPlay`
  ;[1 1 1] BeginPlay
  (set `self.MaxSpeed` 2000.0)
  (set `self.GuidedValue_Yaw` 0.5)
  (set `self.GuidedMaxAngle_Pitch` 5.0)
  (set `self.GuidedValue_Pich` 1.0)
  (set `self.GuidedMaxAngle_Yaw` 2.0))

(event `self.ReceiveTick`
  (params (DeltaSeconds :type "Float (single-precision)"))
  ;[1 1 1] Tick
  (`/Engine/EditorBlueprintResources/StandardMacros.IsValid` self
    (:`Is Valid`
      (bind _outrotator (`/Game/GameAssets/BluePrint/Method/test_method.ConversionAngleTo-180_180` (`self.MoveRotation`)))
      (set `self.MoveRotation` _outrotator)
      (if (`self.ULTMove`)
        (`|ExecutionSequence`
          (:`then_0`
            (`/Engine/EditorBlueprintResources/StandardMacros.DoOnce` false :!label _label
              (:`Completed`
                (`self.LookUp` (`self.K2_GetActorLocation` (`self.Target`))))))
          (:`then_1`
            (`self.UltimateMove` DeltaSeconds)))
        (elif (`/Game/GameAssets/BluePrint/Characters/BP_CharacterBase.IsDead` (`self.Master`))
          (set `self.Fire` false)
          (set `self.FireTimer` 0.0)
          (set `self.IsUnfolding` false)
          (elif (`self.IsAttach`)
            (`self.AttachMove` DeltaSeconds)
            (goto _label :!via `Reset`)
            (else
              (`self.NotAttachMove` DeltaSeconds))))))))

(event `self.DamageCapsule.OnComponentBeginOverlap`
  (params (OverlappedComponent :type "PrimitiveComponent Object Reference") (OtherActor :type "Actor Object Reference") (OtherComp :type "PrimitiveComponent Object Reference") (OtherBodyIndex :type Integer) (bFromSweep :type Boolean) (SweepResult :type "HitResult Structure (by ref)"))
  ;[1 1 1] 当たり判定処理
  (`self.HitCheck` OtherActor OtherComp))

(fn `AttachMove`
  (params (DeltaTIme :type "Float (double-precision)"))
  (locals (NewLocalVar_0 :type Boolean))
  (bind (_returnvalue_roll _returnvalue_pitch _returnvalue_yaw) (`KismetMathLibrary.BreakRotator` (`self.K2_GetActorRotation` (`self.Master`))))
  (bind _asbp_ta_jimaharu (cast `/Game/GameAssets/BluePrint/Characters/ta-jimaharu/BP_ta-jimaharu` (`self.Master`)))
  (set `MovementComponent.Velocity` (0.0 0.0 0.0) (`self.ProjectileMovement`))
  (if (`self.IsUnfolding`)
    (`self.UnfoldingMove` _asbp_ta_jimaharu)
    (`self.LookUp` (`self.K2_GetActorLocation` (`self.Target`)))
    (`self.FireProcess` _asbp_ta_jimaharu)
    (else
      (`self.K2_AddActorWorldOffset` (`KismetMathLibrary.VLerp` (0.0 0.0 0.0) (- (`SceneComponent.GetSocketLocation` (`Character.Mesh` _asbp_ta_jimaharu) (`self.AttachSocketName`)) (`self.K2_GetActorLocation`)) 0.3))
      (`self.K2_SetActorRotation` (`KismetMathLibrary.MakeRotator` _returnvalue_roll 0.0 _returnvalue_yaw)))))

(fn `FireProcess`
  (params (TJM :type "/Game/GameAssets/BluePrint/Characters/ta-jimaharu/BP_ta-jimaharu Object Reference"))
  (if (`self.Fire`)
    (if (> (`self.FireTimer`) 0.0)
      (bind _output_get (set `self.FireTimer` (- (`self.FireTimer`) (`GameplayStatics.GetWorldDeltaSeconds`))))
      (if (<= _output_get 0.0)
        (`/Game/GameAssets/BluePrint/Characters/ta-jimaharu/BP_ta-jimaharu.Sp1BeamShot` TJM (`KismetMathLibrary.Conv_VectorToTransform` (`SceneComponent.K2_GetComponentLocation` (`self.BeamPoint`))))
        (set `self.Fire` false)))
    (else
      (set `self.FireTimer` 0.0))))

(fn `LookUp`
  (params (Location :type "Vector Structure"))
  (`self.K2_SetActorRotation` (`KismetMathLibrary.FindLookAtRotation` (`self.K2_GetActorLocation`) Location)))

(fn `NotAttachMove`
  (params (DeltaTime :type "Float (double-precision)"))
  (if (`self.IsUnfolding`)
    (bind _asbp_ta_jimaharu (cast `/Game/GameAssets/BluePrint/Characters/ta-jimaharu/BP_ta-jimaharu` (`self.Master`)))
    (`self.LookUp` (`self.K2_GetActorLocation` (`self.Target`)))
    (`self.FireProcess` _asbp_ta_jimaharu)
    (elif (`self.Return`)
      (set `MovementComponent.Velocity` (0.0 0.0 0.0) (`self.ProjectileMovement`))
      (set `self.IsGuided` false)
      (else
        (`self.FlightTimeProcess`)
        (`|ExecutionSequence`
          (:`then_0`
            (`self.GoingToMoveDirection` DeltaTime (`self.MaxSpeed`)))
          (:`then_1`
            (if (> (`KismetMathLibrary.DegAcos` (`KismetMathLibrary.Dot_VectorVector` (`self.MoveDirection`) (`self.DirectionToTarget`))) (`self.GuidedAngle`))
              (bind _output_get (set `self.AftertasteTimer` (+ (`self.AftertasteTimer`) DeltaTime)))
              (if (>= _output_get 0.6)
                (set `self.Return` true)
                (set `self.AftertasteTimer` 0.0)
                (`PrimitiveComponent.SetCollisionEnabled` (`self.DamageCapsule`) "NoCollision")
                (`self.K2_SetActorRotation` (struct)))
              (else
                (`self.ChangeDirectionProcessing`)
                (`self.K2_SetActorRotation` (`/Game/GameAssets/BluePrint/Method/BP_MacroLibrary.ConvertRotationUpToForward` (`self.MoveRotation`)))))))))))

(fn `SpawnBeam`
  (bind _target (`self.Target`))
  (bind _returnvalue (`KismetMathLibrary.FindLookAtRotation` (`self.K2_GetActorLocation`) (`self.K2_GetActorLocation` (`self.Target`))))
  (bind _returnvalue_2 (`|SpawnActorFromClass` "/Game/GameAssets/BluePrint/Bullets/Beam/BP_test_beam.BP_test_beam_C" (`KismetMathLibrary.Conv_VectorToTransform` (`SceneComponent.K2_GetComponentLocation` (`self.BeamPoint`))) "Undefined" "OverrideRootScale" null null))
  (bind _asbp_character_base (cast `/Game/GameAssets/BluePrint/Characters/BP_CharacterBase` (`self.Target`)))
  (`/Game/GameAssets/BluePrint/Characters/BP_CharacterBase.FireSeting` _asbp_character_base _returnvalue_2)
  (`|ExecutionSequence`
    (:`then_0`
      (`/Game/GameAssets/BluePrint/Method/BP_MacroLibrary.IsTargetExistence` _target
        (:`NotExistence`
          (`self.K2_SetActorRotation` _returnvalue_2 (`self.K2_GetActorRotation` (`GameplayStatics.GetPlayerController` 0)) false))
        (:`Existence`
          (`self.K2_SetActorRotation` _returnvalue_2 _returnvalue false)
          (set `/Game/GameAssets/BluePrint/Bullets/BP_BuletBase.Target` (`self.Target`) _returnvalue_2))))
    (:`then_1`
      (`/Game/GameAssets/BluePrint/Method/BP_MacroLibrary.IsTargetExistence` _target
        (:`NotExistence`
          (set `/Game/GameAssets/BluePrint/Bullets/BP_BuletBase.MoveRotation` (`self.K2_GetActorRotation`) _returnvalue_2)
          (set `/Game/GameAssets/BluePrint/Bullets/BP_BuletBase.MoveDirection` (`self.GetActorForwardVector` (`GameplayStatics.GetPlayerController` 0)) _returnvalue_2))
        (:`Existence`
          (set `/Game/GameAssets/BluePrint/Bullets/BP_BuletBase.MoveRotation` _returnvalue _returnvalue_2)
          (set `/Game/GameAssets/BluePrint/Bullets/BP_BuletBase.MoveDirection` (`KismetMathLibrary.GetForwardVector` _returnvalue) _returnvalue_2))))
    (:`then_2`
      (set `/Game/GameAssets/BluePrint/Bullets/BP_BuletBase.DamageStruct` (`self.BeamDamage`) _returnvalue_2))))

(fn `UltimateMove`
  (params (DeltaTime :type "Float (double-precision)"))
  (`|ExecutionSequence`
    (:`then_0`
      (if (> (`KismetMathLibrary.DegAcos` (`KismetMathLibrary.Dot_VectorVector` (`self.MoveDirection`) (`self.DirectionToTarget`))) (`self.GuidedAngle`))
        (bind _output_get (set `self.AftertasteTimer` (+ (`self.AftertasteTimer`) DeltaTime)))
        (if (>= _output_get 0.6)
          (set `self.Return` false)
          (set `self.AftertasteTimer` 0.0)
          (set `self.IsAttach` true)
          (set `self.IsUnfolding` false)
          (`PrimitiveComponent.SetCollisionEnabled` (`self.DamageCapsule`) "NoCollision")
          (`self.K2_SetActorRotation` (struct)))
        (else
          (`self.ChangeDirectionProcessing`)
          (`self.K2_SetActorRotation` (`/Game/GameAssets/BluePrint/Method/BP_MacroLibrary.ConvertRotationUpToForward` (`self.MoveRotation`))))))
    (:`then_1`
      (`self.GoingToMoveDirection` DeltaTime (`self.MaxSpeed`)))))

(fn `UnfoldingMove`
  (params (InputPin :type "/Game/GameAssets/BluePrint/Characters/BP_CharacterBase Object Reference"))
  (locals (HorizontallyValue :type "Float (double-precision)" :default 300.0) (`Vertical Value` :type "Float (double-precision)" :default 200.0) (Scale :type "Float (double-precision)" :default 0.7) (Alpha :type "Float (double-precision)" :default 0.2))
  (bind _alpha (`local.Alpha`))
  (bind _alpha_2 (`local.Alpha`))
  (bind (_x _y _z) (`KismetMathLibrary.BreakRotIntoAxes` (`KismetMathLibrary.FindLookAtRotation` (`self.K2_GetActorLocation` InputPin) (`self.K2_GetActorLocation` (`self.Target`)))))
  (switch `/Game/GameAssets/BluePrint/Enum/EN_TJMFunnel` (`self.PositionName`)
    (:`NewEnumerator0`
      (`self.K2_AddActorWorldOffset` (`KismetMathLibrary.VLerp` (0.0 0.0 0.0) (- (+ (* _y (`local.HorizontallyValue`)) (`self.K2_GetActorLocation` InputPin)) (`self.K2_GetActorLocation`)) _alpha_2)))
    (:`NewEnumerator1`
      (`self.K2_AddActorWorldOffset` (`KismetMathLibrary.VLerp` (0.0 0.0 0.0) (- (+ (* _y (* (`local.HorizontallyValue`) (`local.Scale`))) (* _z (`local.Vertical Value`)) (`self.K2_GetActorLocation` InputPin)) (`self.K2_GetActorLocation`)) _alpha_2)))
    (:`NewEnumerator2`
      (`self.K2_AddActorWorldOffset` (`KismetMathLibrary.VLerp` (0.0 0.0 0.0) (- (+ (* _y (`/Game/GameAssets/BluePrint/Method/BP_MacroLibrary.InversFloat` (`local.HorizontallyValue`))) (`self.K2_GetActorLocation` InputPin)) (`self.K2_GetActorLocation`)) _alpha)))
    (:`NewEnumerator3`
      (`self.K2_AddActorWorldOffset` (`KismetMathLibrary.VLerp` (0.0 0.0 0.0) (- (+ (* _y (* (`/Game/GameAssets/BluePrint/Method/BP_MacroLibrary.InversFloat` (`local.HorizontallyValue`)) (`local.Scale`))) (* _z (`local.Vertical Value`)) (`self.K2_GetActorLocation` InputPin)) (`self.K2_GetActorLocation`)) _alpha)))))

(fn `UserConstructionScript`
  (`parent.UserConstructionScript`))