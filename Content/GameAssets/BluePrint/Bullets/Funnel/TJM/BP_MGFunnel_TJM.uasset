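; Machine-gun funnel actor for the ta-jimaharu character (BP_ta-jimaharu) that trails its master and aims at a target.
; It hides itself on BeginPlay.
; Each Tick it moves 30% of the remaining distance toward the AttachSocketName socket on the Master's mesh, giving a frame-rate-dependent eased follow without attachment.
; It also snaps its rotation to face Target whenever that is valid.
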(event `self.ReceiveBeginPlay`
  (`self.SetActorHiddenInGame` true))

(event `self.ReceiveTick`
  (params (DeltaSeconds :type "Float (single-precision)"))
  (bind _target (`self.Target`))
  (bind _master (`self.Master`))
  (`|ExecutionSequence`
    (:`then_0`
      (`/Engine/EditorBlueprintResources/StandardMacros.IsValid` _master
        (:`Is Valid`
          (bind _asbp_ta_jimaharu (cast `/Game/GameAssets/BluePrint/Characters/ta-jimaharu/BP_ta-jimaharu` _master))
          (`self.K2_AddActorWorldOffset` (`KismetMathLibrary.VLerp` (0.0 0.0 0.0) (- (`SceneComponent.GetSocketLocation` (`Character.Mesh` _asbp_ta_jimaharu) (`self.AttachSocketName`)) (`self.K2_GetActorLocation`)) 0.3)))))
    (:`then_1`
      (`/Engine/EditorBlueprintResources/StandardMacros.IsValid` _target
        (:`Is Valid`
          (`self.K2_SetActorRotation` (`KismetMathLibrary.FindLookAtRotation` (`self.K2_GetActorLocation`) (`self.K2_GetActorLocation` _target))))))))

(fn `UserConstructionScript`
  (`parent.UserConstructionScript`))