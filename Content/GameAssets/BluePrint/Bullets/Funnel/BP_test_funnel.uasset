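; Test funnel actor, a drone that homes in on a Target and returns to dock on its Master character.
; Each tick it either eases toward the attach socket with the Master's rotation, or flies along a steered MoveDirection.
; Homing blends direction toward the target until the angle exceeds GuidedAngle, which triggers the return flight.
; It reattaches when near the socket, and LookUp remaps look-at axes to orient it in flight.
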(event `self.ReceiveBeginPlay`
  ;[1 1 1] BeginPlay
  (set `self.MaxSpeed` 2000.0))

(event `self.ReceiveTick`
  (params (DeltaSeconds :type "Float (single-precision)"))
  ;[1 1 1] Tick
  (if (`self.IsAttach`)
    (`self.AttachMove` DeltaSeconds)
    (else
      (`self.NotAttachMove` DeltaSeconds))))

(fn `AttachMove`
  (params (DeltaTIme :type "Float (double-precision)"))
  (locals (NewLocalVar_0 :type Boolean))
  (bind _asbp_character_base (cast `/Game/GameAssets/BluePrint/Characters/BP_CharacterBase` (`self.Master`)))
  (`self.K2_AddActorWorldOffset` (`KismetMathLibrary.VLerp` (0.0 0.0 0.0) (- (`SceneComponent.GetSocketLocation` (`Character.Mesh` _asbp_character_base) (`self.AttachSocketName`)) (`self.K2_GetActorLocation`)) 0.2))
  (`self.K2_SetActorRotation` (`self.K2_GetActorRotation` (`self.Master`))))

(fn `GoingToMoveDirection`
  (params (DeltaTime :type "Float (double-precision)") (Speed :type "Float (double-precision)"))
  (`self.K2_AddActorWorldTransform` (`KismetMathLibrary.Conv_VectorToTransform` (* (`self.MoveDirection`) (* DeltaTime Speed)))))

(fn `LookUp`
  (params (Location :type "Vector Structure"))
  (bind (_x _y _z) (`KismetMathLibrary.BreakRotIntoAxes` (`KismetMathLibrary.FindLookAtRotation` (`self.K2_GetActorLocation`) Location)))
  (`self.K2_SetActorRotation` (`KismetMathLibrary.MakeRotationFromAxes` _z _y (* _x -1))))

(fn `NotAttachMove`
  (params (DeltaTime :type "Float (double-precision)"))
  (bind _direction (`self.DirectionToTarget`))
  (bind _movedirection (`self.MoveDirection`))
  (bind _attachsocketname (`self.AttachSocketName`))
  (if (`self.Return`)
    (bind _asbp_character_base (cast `/Game/GameAssets/BluePrint/Characters/BP_CharacterBase` (`self.Master`)))
    (bind _mesh (`Character.Mesh` _asbp_character_base))
    (if (`SceneComponent.DoesSocketExist` _mesh _attachsocketname)
      (`|ExecutionSequence`
        (:`then_0`
          (bind _returnvalue (`SceneComponent.GetSocketLocation` _mesh _attachsocketname))
          (bind _returnvalue_2 (- _returnvalue (`self.K2_GetActorLocation`)))
          (set `self.MoveDirection` (`KismetMathLibrary.Normal` (`KismetMathLibrary.VLerp` (`self.MoveDirection`) (`KismetMathLibrary.Normal` _returnvalue_2) 0.25))))
        (:`then_1`
          (`self.GoingToMoveDirection` DeltaTime (`self.ReturnSpeed`))
          (`self.LookUp` _returnvalue)
          (if (< (`KismetMathLibrary.VSize` _returnvalue_2) 20.0)
            (set `self.Return` false)
            (set `self.IsAttach` true)))))
    (else
      (`|ExecutionSequence`
        (:`then_0`
          (`self.GoingToMoveDirection` DeltaTime (`self.MaxSpeed`))
          (if (not (`self.Aftertaste`))
            (`self.LookUp` (`self.K2_GetActorLocation` (`self.Target`)))))
        (:`then_1`
          (`self.IsTargetExistence`
            (:`Existence`
              (set `self.MoveDirection` (`KismetMathLibrary.Normal` (`KismetMathLibrary.VLerp` _movedirection _direction (`self.GuidedValue_Yaw`))))
              (if (> (`KismetMathLibrary.DegAcos` (`KismetMathLibrary.Dot_VectorVector` _movedirection _direction)) (`self.GuidedAngle`))
                (set `self.Aftertaste` true)
                (set `self.Return` true)))))))))

(fn `UserConstructionScript`)