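; BP_ULTExplosion_TJM is a stationary ultimate explosion that repeatedly damages characters inside its expanding area until its flight time expires.
; Each tick grows DamageCapsule's radius and half-height up to a maximum.
; Its collision switches on for one tick per hit interval, counted in frames, to re-trigger overlaps.
; Overlaps with components tagged HitCapsule on BP_CharacterBase actors call DamageServer.
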(event `self.ReceiveBeginPlay`
  (set `self.FlightTime` 4.0)
  (set `MovementComponent.Velocity` (0.0 0.0 0.0) (`self.ProjectileMovement`)))

(event `self.ReceiveTick`
  (params (DeltaSeconds :type "Float (single-precision)"))
  (bind _damagecapsule (`self.DamageCapsule`))
  (`self.FlightTimeProcess`)
  (`|ExecutionSequence`
    (:`then_0`
      (bind _output_get (set `self.DamageSize` (`KismetMathLibrary.FClamp` (+ (`self.DamageSize`) (* (`self.EnlargementSpeed`) DeltaSeconds)) 0.0 (`self.DamageMaxSize`))))
      (`CapsuleComponent.SetCapsuleHalfHeight` _damagecapsule _output_get true)
      (`CapsuleComponent.SetCapsuleRadius` _damagecapsule _output_get true))
    (:`then_1`
      (if (<= (`self.HitIntervalTimer`) 0.0)
        (set `self.HitIntervalTimer` (`self.HitInterval`))
        (`PrimitiveComponent.SetCollisionEnabled` (`self.DamageCapsule`) "QueryOnly")
        (else
          (set `self.HitIntervalTimer` (- (`self.HitIntervalTimer`) 1.0))
          (`PrimitiveComponent.SetCollisionEnabled` (`self.DamageCapsule`) "NoCollision"))))
    (:`then_2`
      (if (<= (`self.FlightTime`) 0.0)
        (`self.K2_DestroyActor`)))))

(event `self.DamageCapsule.OnComponentBeginOverlap`
  (params (OverlappedComponent :type "PrimitiveComponent Object Reference") (OtherActor :type "Actor Object Reference") (OtherComp :type "PrimitiveComponent Object Reference") (OtherBodyIndex :type Integer) (bFromSweep :type Boolean) (SweepResult :type "HitResult Structure (by ref)"))
  (`self.HitCheck` OtherActor OtherComp))

(fn `HitCheck`
  (params (Actor :type "Object Object Reference") (Component :type "Object Object Reference"))
  (bind _ascapsule_collision (cast `CapsuleComponent` Component))
  (for _array_element (`ActorComponent.ComponentTags` _ascapsule_collision)
    (if (== _array_element "HitCapsule")
      (bind _asbp_character_base (cast `/Game/GameAssets/BluePrint/Characters/BP_CharacterBase` Actor))
      (`self.DamageServer` _asbp_character_base))))

(fn `UserConstructionScript`
  (`parent.UserConstructionScript`))