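; BP_MG_TJM is a guided projectile in the MG bullet set that homes by changing its travel direction in flight.
; BeginPlay sets its max speed and yaw/pitch guidance values and angle limits, with a wider limit on yaw than pitch.
; Each Tick wraps rotation to ±180°, destroys the actor when its flight time expires, moves it, then updates steering.
; Overlaps on the damage capsule run the hit check.
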(event `self.ReceiveBeginPlay`
  (set `self.MaxSpeed` 2400.0)
  (`|ExecutionSequence`
    (:`then_0`
      (set `self.GuidedValue_Yaw` 1.0)
      (set `self.GuidedValue_Pich` 1.0))
    (:`then_1`
      (set `self.GuidedMaxAngle_Pitch` 5.0)
      (set `self.GuidedMaxAngle_Yaw` 10.0))))

(event `self.ReceiveTick`
  (params (DeltaSeconds :type "Float (single-precision)"))
  (bind _outrotator (`/Game/GameAssets/BluePrint/Method/test_method.ConversionAngleTo-180_180` (`self.MoveRotation`)))
  (set `self.MoveRotation` _outrotator)
  (`|ExecutionSequence`
    (:`then_0`
      ;[1 1 1] 射程（時間）がきたら消す
      (bind _destroy (`self.FightTImeProcessing` DeltaSeconds))
      (if _destroy
        (`self.K2_DestroyActor`)))
    (:`then_1`
      ;[1 1 1] 移動処理
      (`self.Move` DeltaSeconds))
    (:`then_2`
      ;[1 1 1] 誘導する動き（進む方向を変える）
      (`self.ChangeDirectionProcessing`))))

(event `self.DamageCapsule.OnComponentBeginOverlap`
  (params (OverlappedComponent :type "PrimitiveComponent Object Reference") (OtherActor :type "Actor Object Reference") (OtherComp :type "PrimitiveComponent Object Reference") (OtherBodyIndex :type Integer) (bFromSweep :type Boolean) (SweepResult :type "HitResult Structure (by ref)"))
  ;[1 1 1] Hit判定
  (`self.HitCheck` OtherActor OtherComp))

(fn `UserConstructionScript`
  (`parent.UserConstructionScript`))