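; BP_BuletBase is a bullet base Blueprint providing straight movement, limited homing and a flight-time countdown.
; Move offsets the actor along MoveDirection at MaxSpeed without sweeping, while FightTImeProcessing reports when FlightTime runs out.
; ChangeDirectionProcessing checks that a Target exists and lies within GuidedAngle, then lerps MoveDirection toward it by GuidedValue and renormalizes.
; No event here calls these functions.
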(fn `ChangeDirectionProcessing`
  (bind _direction (`self.DirectionToTarget`))
  (bind _movedirection (`self.MoveDirection`))
  (`self.IsTargetExistence`
    (:`Existence`
      (if (not (> (`KismetMathLibrary.DegAcos` (`KismetMathLibrary.Dot_VectorVector` _movedirection _direction)) (`self.GuidedAngle`)))
        (set `self.MoveDirection` (`KismetMathLibrary.Normal` (`KismetMathLibrary.VLerp` _movedirection _direction (`self.GuidedValue`))))))))

(fn `FightTImeProcessing`
  (params (DeltaTime :type "Float (double-precision)"))
  (returns (Destroy :type Boolean))
  (bind _output_get (set `self.FlightTime` (- (`self.FlightTime`) DeltaTime)))
  (return (<= _output_get 0.0)))

(fn `Move`
  (params (DeltaTime :type "Float (double-precision)"))
  (`self.K2_AddActorWorldTransform` (`KismetMathLibrary.Conv_VectorToTransform` (* (`self.MoveDirection`) (* DeltaTime (`self.MaxSpeed`))))))

(fn `UserConstructionScript`)