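; BP_Warhead_TJM is a homing warhead projectile that spawns BP_ULTExplosion_TJM on impact.
; After a start delay, it steers yaw and pitch toward its Target; a second timer clears IsGuided, but Guid stays set, so steering continues.
; Overlapping a HitCapsule, except on same-ConsortPlaneValue characters, or hitting a BulletBlocker triggers a one-time ExplosionServer.
; That event passes the explosion to the Attacker for damage setup, then destroys the warhead.
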(event `self.ReceiveBeginPlay`
  (set `self.MaxSpeed` 2400.0)
  (set `self.GuidedValue_Yaw` 1.0)
  (set `self.GuidedMaxAngle_Pitch` 5.0)
  (set `self.GuidedValue_Pich` 0.5)
  (set `self.GuidedMaxAngle_Yaw` 5.0)
  (set `self.StartTimer` 2.0)
  (set `self.IsGuided` true)
  (set `self.GuidedTimer` 1.0)
  (set `self.Guid` false))

(event `self.ReceiveTick`
  (params (DeltaSeconds :type "Float (single-precision)"))
  (bind _outrotator (`/Game/GameAssets/BluePrint/Method/test_method.ConversionAngleTo-180_180` (`self.MoveRotation`)))
  (set `self.MoveRotation` _outrotator)
  (`|ExecutionSequence`
    (:`then_0`
      (if (> (`self.StartTimer`) 0.0)
        (bind _output_get (set `self.StartTimer` (- (`self.StartTimer`) DeltaSeconds)))
        (if (<= _output_get 0.0)
          (set `self.IsGuided` true)
          (set `self.Guid` true))))
    (:`then_1`
      (`self.ChangeDirectionProcessing`)
      ;[1 1 1] 一度角度が合えば誘導しなくなる
      (if (and (> (`self.GuidedTimer`) 0.0) (<= (`self.StartTimer`) 0.0))
        (bind _output_get_2 (set `self.GuidedTimer` (- (`self.GuidedTimer`) DeltaSeconds)))
        (if (<= _output_get_2 0.0)
          (set `self.IsGuided` false)
          (set `self.Guid` true))))
    (:`then_2`
      (`self.Move` DeltaSeconds)
      (`self.K2_SetActorRotation` (`/Game/GameAssets/BluePrint/Method/BP_MacroLibrary.ConvertRotationUpToForward` (`self.MoveRotation`))))
    (:`then_3`
      (`KismetSystemLibrary.PrintString` "Hello" true true (struct :`G` 0.66 :`B` 1.0 :`A` 1.0) 0.1))))

(event `self.DamageCapsule.OnComponentBeginOverlap`
  (params (OverlappedComponent :type "PrimitiveComponent Object Reference") (OtherActor :type "Actor Object Reference") (OtherComp :type "PrimitiveComponent Object Reference") (OtherBodyIndex :type Integer) (bFromSweep :type Boolean) (SweepResult :type "HitResult Structure (by ref)"))
  (if (!= (`self.ConsortPlaneValue`) -1)
    (bind _ascapsule_collision (cast `CapsuleComponent` OtherComp))
    (for _array_element (`ActorComponent.ComponentTags` _ascapsule_collision)
      (if (== _array_element "HitCapsule")
        (bind _asbp_character_base (cast `/Game/GameAssets/BluePrint/Characters/BP_CharacterBase` OtherActor)
          (:`then`
            (if (!= (`self.ConsortPlaneValue`) (`/Game/GameAssets/BluePrint/Characters/BP_CharacterBase.ConsortPlaneValue` _asbp_character_base))
              (`self.ExplosionServer` :!label _label)))
          (:`CastFailed`
            (goto _label)))))))

(event `self.DamageCapsule.OnComponentHit`
  (params (HitComponent :type "PrimitiveComponent Object Reference") (OtherActor :type "Actor Object Reference") (OtherComp :type "PrimitiveComponent Object Reference") (NormalImpulse :type "Vector Structure") (Hit :type "HitResult Structure (by ref)"))
  (if (`self.ActorHasTag` OtherActor "BulletBlocker")
    (goto _label)))

(event `ExplosionServer`
  (bind _attacker (`self.Attacker`))
  (`/Engine/EditorBlueprintResources/StandardMacros.DoOnce` false
    (:`Completed`
      (bind _returnvalue (`|SpawnActorFromClass` "/Game/GameAssets/BluePrint/Bullets/Explosion/BP_ULTExplosion_TJM.BP_ULTExplosion_TJM_C" (`self.GetTransform`) "Undefined" "OverrideRootScale" null null))
      (`/Game/GameAssets/BluePrint/Characters/BP_CharacterBase.FireSeting` _attacker _returnvalue)
      (set `/Game/GameAssets/BluePrint/Bullets/BP_BuletBase.ConsortPlaneValue` -1 _returnvalue)
      (set `/Game/GameAssets/BluePrint/Bullets/BP_BuletBase.IsGuided` false _returnvalue)
      (`/Game/GameAssets/BluePrint/Characters/BP_CharacterBase.SetSelectStageDamageProcess` _attacker 1 _returnvalue "NewEnumerator4")
      (`self.K2_DestroyActor`))))

(fn `ChangeDirectionProcessing`
  (bind (_moverotation_roll _moverotation_pitch _moverotation_yaw) (`KismetMathLibrary.BreakRotator` (`self.MoveRotation`)))
  (if (`self.Guid`)
    (`self.IsTargetExistence`
      (:`Existence`
        (bind _revolutionyawangle (`self.YawAngleValue`))
        (bind _revolutionpitchangle (`self.PitchAngleValue`))
        (bind _output_get (set `self.MoveRotation` (`KismetMathLibrary.MakeRotator` 0.0 (+ _revolutionpitchangle _moverotation_pitch) (+ _revolutionyawangle _moverotation_yaw))))
        (set `self.MoveDirection` (`KismetMathLibrary.GetForwardVector` _output_get))))))

(fn `UserConstructionScript`
  (`parent.UserConstructionScript`))