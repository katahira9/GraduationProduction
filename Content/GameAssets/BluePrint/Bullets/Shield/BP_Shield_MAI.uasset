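; BP_Shield_MAI is a shield actor, filed under Bullets, that rises from its spawn point and damages characters on another ConsortPlaneValue.
; Tick moves it up by UpValue over UpTIme and starts a one-second Delay that destroys it.
; The damage capsule's collision switches on once ConsortPlaneValue is set.
; Overlaps go through HitCheck, which requires a HitCapsule-tagged capsule on a BP_CharacterBase before calling DamageServer.
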(event `self.ReceiveBeginPlay`
  (set `self.Point` (`self.K2_GetActorLocation`)))

(event `self.ReceiveTick`
  (params (DeltaSeconds :type "Float (single-precision)"))
  (bind _uptimer (`self.UpTimer`))
  (bind _uptime (`self.UpTIme`))
  (`|ExecutionSequence`
    (:`then_0`
      (if (!= (`self.ConsortPlaneValue`) -1)
        (`/Engine/EditorBlueprintResources/StandardMacros.DoOnce` false
          (:`Completed`
            (`PrimitiveComponent.SetCollisionEnabled` (`self.DamageCapsule`) "QueryAndPhysics")))))
    (:`then_1`
      (if (< _uptimer _uptime)
        (set `self.UpTimer` (`KismetMathLibrary.FClamp` (+ _uptimer DeltaSeconds) 0.0 _uptime))
        (`self.K2_SetActorLocation` (+ (`KismetMathLibrary.MakeVector` 0.0 0.0 (* (`self.UpValue`) (/ (`self.UpTimer`) (`self.UpTIme`)))) (`self.Point`)))
        (`KismetSystemLibrary.Delay` 1.0)
        (`self.K2_DestroyActor`)))))

(event `self.DamageCapsule.OnComponentBeginOverlap`
  (params (OverlappedComponent :type "PrimitiveComponent Object Reference") (OtherActor :type "Actor Object Reference") (OtherComp :type "PrimitiveComponent Object Reference") (OtherBodyIndex :type Integer) (bFromSweep :type Boolean) (SweepResult :type "HitResult Structure (by ref)"))
  ;[1 1 1] Hit判定
  (`self.HitCheck` OtherActor OtherComp))

(fn `HitCheck`
  (params (Actor :type "Object Object Reference") (Component :type "Object Object Reference"))
  (bind _ascapsule_collision (cast `CapsuleComponent` Component))
  (for _array_element (`ActorComponent.ComponentTags` _ascapsule_collision)
    (if (== _array_element "HitCapsule")
      (bind _asbp_character_base (cast `/Game/GameAssets/BluePrint/Characters/BP_CharacterBase` Actor))
      (if (!= (`self.ConsortPlaneValue`) (`/Game/GameAssets/BluePrint/Characters/BP_CharacterBase.ConsortPlaneValue` _asbp_character_base))
        (`self.DamageServer` _asbp_character_base)))))

(fn `UserConstructionScript`
  (`parent.UserConstructionScript`))