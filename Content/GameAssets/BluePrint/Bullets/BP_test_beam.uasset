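; BP_test_beam is a test beam projectile that flies with homing movement and damages characters it hits.
; Each tick it destroys itself once its time-based range runs out, moves, then adjusts its heading toward homing.
; Sphere overlaps pass the damage struct through DamageServer to any BP_CharacterBase whose ConsortPlaneValue differs from its own, unless its own is -1.
; Movement, lifetime and steering functions are called but not defined here.
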(event `self.ReceiveTick`
  (params (DeltaSeconds :type "Float (single-precision)"))
  (set `self.MoveRotation` (`self.K2_GetActorRotation`))
  (`|ExecutionSequence`
    (:`then_0`
      ;[1 1 1] 射程（時間）がきたら消す
      (bind _destroy (`self.FightTImeProcessing` DeltaSeconds))
      (if _destroy
        (`self.K2_DestroyActor`)))
    (:`then_1`
      ;[1 1 1] 移動処理
      (`self.Move` DeltaSeconds))
    (:`then_2`
      ;[1 1 1] 誘導する動き（進む方向を変える）
      (`self.ChangeDirectionProcessing`))))

(event `self.Sphere.OnComponentBeginOverlap`
  (params (OverlappedComponent :type "PrimitiveComponent Object Reference") (OtherActor :type "Actor Object Reference") (OtherComp :type "PrimitiveComponent Object Reference") (OtherBodyIndex :type Integer) (bFromSweep :type Boolean) (SweepResult :type "HitResult Structure (by ref)"))
  (if (!= (`self.ConsortPlaneValue`) -1)
    (bind _asbp_character_base (cast `/Game/GameAssets/BluePrint/Characters/BP_CharacterBase` OtherActor))
    (if (!= (`self.ConsortPlaneValue`) (`/Game/GameAssets/BluePrint/Characters/BP_CharacterBase.ConsortPlaneValue` _asbp_character_base))
      (`self.DamageServer` _asbp_character_base))))

(event `DamageServer`
  (params (Character :type "/Game/GameAssets/BluePrint/Characters/BP_CharacterBase Object Reference"))
  (`/Game/GameAssets/BluePrint/Characters/BP_CharacterBase.DamageEvent` Character (`self.DamageStruct`)))

(fn `UserConstructionScript`
  (`parent.UserConstructionScript`))