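; Missile-pod bullet that homes on a target, expires after its time-based range and is destroyed on hitting BulletBlocker actors.
; Tick drives ProjectileMovement along MoveDirection, rotated toward the target by a capped cross-product axis-angle turn.
; A repeating short Delay re-enables guidance, while exceeding the guidance angle disables it.
; "Funny" missiles aim at a once-rolled random offset from the target; capsule overlaps go to HitCheck.
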(event `SetGuideServer`
  (params (Guided :type Boolean))
  (set `self.IsGuided` Guided))

(event `self.ReceiveBeginPlay`
  (set `self.MaxSpeed` 4000.0)
  (set `self.GuidedValue_Yaw` 1.0)
  (set `self.GuidedMaxAngle_Pitch` 0.5)
  (set `self.GuidedValue_Pich` 30.0)
  (set `self.GuidedMaxAngle_Yaw` 30.0)
  (set `self.GuidedAngle` 70.0)
  (set `self.bIsMissile` true))

(event `self.ReceiveTick`
  (params (DeltaSeconds :type "Float (single-precision)"))
  (set `self.MoveRotation` (`self.K2_GetActorRotation`))
  (`|ExecutionSequence`
    (:`then_0`
      (`/Engine/EditorBlueprintResources/StandardMacros.DoOnce` false
        (:`Completed`
          (if (`self.IsFunnyMissile`)
            (bind _newparam (`self.DisideFunnyVec`))
            (set `self.Vector` _newparam)))))
    (:`then_1`
      ;[1 1 1] 射程（時間）がきたら消す
      (bind _destroy (`self.FightTImeProcessing` DeltaSeconds))
      (if _destroy
        (`self.K2_DestroyActor`)))
    (:`then_2`
      ;[1 1 1] 移動処理
      (`self.Move` DeltaSeconds))
    (:`then_3`
      ;[1 1 1] 誘導する動き（進む方向を変える）
      (`self.ChangeDirectionProcessing`))
    (:`then_4`
      (`KismetSystemLibrary.Delay` 0.1)
      (set `self.IsGuided` true))
    (:`then_5`
      (if (> (`KismetMathLibrary.DegAcos` (`KismetMathLibrary.Dot_VectorVector` (`self.MoveDirection`) (`self.DirectionToTarget`))) (`self.GuidedAngle`))
        (set `self.IsGuided` false)))))

(event `self.DamageCapsule.OnComponentHit`
  (params (HitComponent :type "PrimitiveComponent Object Reference") (OtherActor :type "Actor Object Reference") (OtherComp :type "PrimitiveComponent Object Reference") (NormalImpulse :type "Vector Structure") (Hit :type "HitResult Structure (by ref)"))
  ;[1 1 1] ブロック判定
  (if (`self.ActorHasTag` OtherActor "BulletBlocker")
    (`self.K2_DestroyActor`)))

(event `self.DamageCapsule.OnComponentBeginOverlap`
  (params (OverlappedComponent :type "PrimitiveComponent Object Reference") (OtherActor :type "Actor Object Reference") (OtherComp :type "PrimitiveComponent Object Reference") (OtherBodyIndex :type Integer) (bFromSweep :type Boolean) (SweepResult :type "HitResult Structure (by ref)"))
  (`self.HitCheck` OtherActor OtherComp))

(fn `ChangeDirectionProcessing`
  (bind (_moverotation_roll _moverotation_pitch _moverotation_yaw) (`KismetMathLibrary.BreakRotator` (`self.MoveRotation`)))
  (bind _returnvalue (`KismetMathLibrary.Normal` (`self.MoveDirection`)))
  (bind _returnvalue_2 (`KismetMathLibrary.Normal` (`self.MoveDirection`)))
  (bind _returnvalue_3 (`KismetMathLibrary.Normal` (- (`self.K2_GetActorLocation` (`self.Target`)) (`self.K2_GetActorLocation`))))
  (bind _returnvalue_4 (`KismetMathLibrary.Cross_VectorVector` _returnvalue _returnvalue_3))
  (bind _returnvalue_5 (`KismetMathLibrary.Normal` (- (+ (`self.Vector`) (`self.K2_GetActorLocation` (`self.Target`))) (`self.K2_GetActorLocation`))))
  (bind _returnvalue_6 (`KismetMathLibrary.Cross_VectorVector` _returnvalue_2 _returnvalue_5))
  (bind _returnvalue_7 (`KismetMathLibrary.VSize` _returnvalue_4))
  (bind _returnvalue_8 (`KismetMathLibrary.VSize` _returnvalue_6))
  (if (`self.IsGuided`)
    (bind _bool (`self.IsWithinGuidedAngle`))
    (if _bool
      (bind _revolutionyawangle (`self.YawAngleValue`))
      (bind _revolutionpitchangle (`self.PitchAngleValue`))
      (set `self.MoveRotation` (`KismetMathLibrary.MakeRotator` 0.0 (+ _revolutionpitchangle _moverotation_pitch) (+ _revolutionyawangle _moverotation_yaw)))
      (if (`self.IsFunnyMissile`)
        (if (!= _returnvalue_8 0.0)
          (set `self.MoveDirection` (`KismetMathLibrary.GreaterGreater_VectorRotator` (`self.MoveDirection`) (`KismetMathLibrary.RotatorFromAxisAndAngle` (/ _returnvalue_6 _returnvalue_8) (`KismetMathLibrary.FMin` (`KismetMathLibrary.DegAcos` (`KismetMathLibrary.Dot_VectorVector` _returnvalue_5 _returnvalue_2)) (* (`self.RotateBySec`) (`GameplayStatics.GetWorldDeltaSeconds`)))))))
        (elif (!= _returnvalue_7 0.0)
          (set `self.MoveDirection` (`KismetMathLibrary.GreaterGreater_VectorRotator` (`self.MoveDirection`) (`KismetMathLibrary.RotatorFromAxisAndAngle` (/ _returnvalue_4 _returnvalue_7) (`KismetMathLibrary.FMin` (`KismetMathLibrary.DegAcos` (`KismetMathLibrary.Dot_VectorVector` _returnvalue_3 _returnvalue)) (* (`self.RotateBySec`) (`GameplayStatics.GetWorldDeltaSeconds`))))))))
      (else
        (set `self.IsGuided` false)))))

(fn `DisideFunnyVec`
  (returns (NewParam :type "Vector Structure"))
  (bind _target (`self.Target`))
  (return (+ (* (`self.GetActorForwardVector` _target) (`KismetMathLibrary.RandomFloatInRange` (`self.MIN`) (`self.MAX`))) (* (`self.GetActorUpVector` _target) (`KismetMathLibrary.RandomFloatInRange` (`self.MIN`) (`self.MAX`))) (* (`self.GetActorRightVector` _target) (`KismetMathLibrary.RandomFloatInRange` (`self.MIN`) (`self.MAX`))))))

(fn `Move`
  (params (DeltaTime :type "Float (double-precision)"))
  (bind _projectilemovement (`self.ProjectileMovement`))
  (`/Engine/EditorBlueprintResources/StandardMacros.IsValid` _projectilemovement
    (:`Is Valid`
      (set `MovementComponent.Velocity` (* (`KismetMathLibrary.Normal` (`self.MoveDirection`)) (`self.MaxSpeed`)) _projectilemovement))))

(fn `UserConstructionScript`
  (`parent.UserConstructionScript`))