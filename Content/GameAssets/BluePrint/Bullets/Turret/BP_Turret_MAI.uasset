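; Turret actor for the Moai character (BP_Moai) that faces its owner's target and fires shots through the owner's attack functions.
; In normal mode, a fire order triggers a timed shot via MAIAttack2Shot, and the turret expires when flight time or uses run out.
; In ULT mode, after a standby delay, it orbits above the target, calling MAIULTShot at intervals until the ULT timer ends.
; Aiming zeroes pitch, keeping the turret level.
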(event `self.ReceiveBeginPlay`
  ;[1 1 1] Begin Play
  (set `self.FlightTime` 60.0)
  (set `self.IsGuided` false))

(event `ULTFireTimerProcessServer`
  ;[1 1 1] カスタムイベント
  (if (<= (`self.ULTFireTimer`) 0.0)
    (bind _asbp_moai (cast `/Game/GameAssets/BluePrint/Characters/moai/BP_Moai` (`self.Attacker`)))
    (`/Game/GameAssets/BluePrint/Characters/moai/BP_Moai.MAIULTShot` _asbp_moai (`SceneComponent.K2_GetComponentLocation` (`self.ShotPoint`)))))

(event `FireOderServer`
  ;[1 1 1] カスタムイベント
  (set `self.FireOder` true))

(event `self.ReceiveTick`
  (params (DeltaSeconds :type "Float (single-precision)"))
  (bind _attacker (`self.Attacker`))
  (bind _target (`self.Target`))
  (bind (_returnvalue_roll _returnvalue_pitch _returnvalue_yaw) (`KismetMathLibrary.BreakRotator` (`KismetMathLibrary.FindLookAtRotation` (`self.K2_GetActorLocation`) (`self.K2_GetActorLocation` _target))))
  ;[1 1 1] Tick
  (`|ExecutionSequence`
    (:`then_0`
      (`/Engine/EditorBlueprintResources/StandardMacros.IsValid` _attacker
        (:`Is Valid`
          (set `self.Target` (`/Game/GameAssets/BluePrint/Characters/BP_CharacterBase.Target` _attacker))
          (`self.LifeSpanProcess`))))
    (:`then_1`
      (if (`self.bisULT`)
        (`self.ULTProcess` DeltaSeconds)
        (else
          (`/Engine/EditorBlueprintResources/StandardMacros.IsValid` _target
            (:`Is Valid`
              (`self.K2_SetActorRotation` (`KismetMathLibrary.MakeRotator` _returnvalue_roll 0.0 _returnvalue_yaw)))))))
    (:`then_2`
      (`self.ShotOderProcess` DeltaSeconds))))

(fn `LifeSpanProcess`
  (if (not (`self.bisULT`))
    (`|ExecutionSequence`
      (:`then_0`
        (`self.FlightTimeProcess`)
        (if (<= (`self.FlightTime`) 0.0)
          (`self.K2_DestroyActor`)))
      (:`then_1`
        (if (<= (`self.UseCount`) 0)
          (`self.K2_DestroyActor`))))))

(fn `ShotOderProcess`
  (params (DT :type "Float (double-precision)"))
  (if (`self.FireOder`)
    (bind _output_get (set `self.FireTimer` (- (`self.FireTimer`) DT)))
    (if (<= _output_get 0.0)
      (bind _asbp_moai (cast `/Game/GameAssets/BluePrint/Characters/moai/BP_Moai` (`self.Attacker`)))
      (`/Game/GameAssets/BluePrint/Characters/moai/BP_Moai.MAIAttack2Shot` _asbp_moai (`SceneComponent.K2_GetComponentLocation` (`self.ShotPoint`)))
      (set `self.FireOder` false)
      (`/Engine/EditorBlueprintResources/StandardMacros.DecrementInt` (`self.UseCount`)))))

(fn `ULTProcess`
  (params (TD :type "Float (double-precision)"))
  (locals (ULTFireTime :type "Float (double-precision)" :default 2.0))
  (bind _target (`self.Target`))
  (bind _ultangle (`self.ULTAngle`))
  (bind _target_2 (`self.Target`))
  (bind _ultfiretimer (`self.ULTFireTimer`))
  (bind _ultstandbytimer (`self.ULTStandbyTimer`))
  (bind _distance (`self.Distance`))
  (bind (_returnvalue_roll _returnvalue_pitch _returnvalue_yaw) (`KismetMathLibrary.BreakRotator` (`KismetMathLibrary.FindLookAtRotation` (`self.K2_GetActorLocation`) (`self.K2_GetActorLocation` _target_2))))
  (if (> _ultstandbytimer 0.0)
    (set `self.ULTStandbyTimer` (- _ultstandbytimer TD))
    (else
      (`|ExecutionSequence`
        (:`then_0`
          (`/Engine/EditorBlueprintResources/StandardMacros.IsValid` _target_2
            (:`Is Valid`
              (`self.K2_SetActorRotation` (`KismetMathLibrary.MakeRotator` _returnvalue_roll 0.0 _returnvalue_yaw)))))
        (:`then_1`
          (bind _output_get (set `self.ULTAngle` (+ (`self.ULTAngle`) (* (`self.AngleSpeed`) TD))))
          (if (> _output_get 360.0)
            (set `self.ULTAngle` (- _output_get 360.0)))
          (`/Engine/EditorBlueprintResources/StandardMacros.IsValid` _target
            (:`Is Valid`
              (`self.K2_SetActorLocation` (+ (`self.K2_GetActorLocation` _target) (`KismetMathLibrary.MakeVector` (* (`KismetMathLibrary.DegSin` _ultangle) _distance) (* _distance (`KismetMathLibrary.DegCos` _ultangle)) 100.0))))))
        (:`then_2`
          (if (> _ultfiretimer 0.0)
            (set `self.ULTFireTimer` (- _ultfiretimer TD))
            (`self.ULTFireTimerProcessServer`)
            (else
              (set `self.ULTFireTimer` (`local.ULTFireTime`)))))
        (:`then_3`
          (bind _output_get_2 (set `self.ULTTimer` (- (`self.ULTTimer`) TD)))
          (if (<= _output_get_2 0.0)
            (`self.K2_DestroyActor`)))))))

(fn `UserConstructionScript`
  (`parent.UserConstructionScript`))