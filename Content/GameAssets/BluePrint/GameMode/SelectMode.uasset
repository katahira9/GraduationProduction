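; SelectMode is the game mode for a pre-game selection stage that assigns players and starts the match when everyone is ready.
; PostLogin gives each BP_PlayerState an incrementing player number and a team ID alternating between two teams.
; Tick polls the ReadyStruct entries in BP_GameState and runs a ServerTravel to the Game map once all are true and the next player number is at least four.
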(event `self.K2_PostLogin`
  (params (NewPlayer :type "PlayerController Object Reference"))
  (bind _nextteamid (`self.NextTeamID`))
  (bind _asbp_player_state (cast `/Game/GameAssets/BluePrint/PlayerState/BP_PlayerState` (`Controller.PlayerState` NewPlayer)))
  (`|ExecutionSequence`
    (:`then_0`
      (set `/Game/GameAssets/BluePrint/PlayerState/BP_PlayerState.PlayerNumber` (`self.NextPlayerNumber`) _asbp_player_state)
      (bind _result (`/Engine/EditorBlueprintResources/StandardMacros.IncrementInt` (`self.NextPlayerNumber`))
        (:`  `
          (set `self.NextPlayerNumber` _result))))
    (:`then_1`
      (set `/Game/GameAssets/BluePrint/PlayerState/BP_PlayerState.TeamID` (`self.NextTeamID`) _asbp_player_state)
      (`/Engine/EditorBlueprintResources/StandardMacros.IncrementInt` _nextteamid
        (:`  `
          (set `self.NextTeamID` (mod _nextteamid 2)))))))

(event `self.ReceiveTick`
  (params (DeltaSeconds :type "Float (single-precision)"))
  (set `self.MoveFlug` false)
  (`|ExecutionSequence`
    (:`then_0`
      (bind _asbp_game_state (cast `/Game/GameAssets/BluePrint/GameState/BP_GameState` (`GameplayStatics.GetGameState`)))
      (for _array_element (`/Game/GameAssets/BluePrint/GameState/BP_GameState.ReadyStruct` _asbp_game_state)
        (if _array_element
          (set `self.MoveFlug` true)
          (else
            (set `self.MoveFlug` false)
            (break)))))
    (:`then_1`
      (if (`self.MoveFlug`)
        (if (>= (`self.NextPlayerNumber`) 4)
          (`KismetSystemLibrary.ExecuteConsoleCommand` "ServerTravel Game" null))))))

(fn `UserConstructionScript`)