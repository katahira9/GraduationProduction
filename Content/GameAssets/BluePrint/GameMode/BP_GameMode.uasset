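; Game mode that assigns players to two teams and decides which team has won.
; On login it gives each player state an incrementing player number and an alternating team ID.
; Every tick it reads both team costs from the game state and, when one reaches zero, sets the other team as winner there.
; When the player counter drops to zero on logout in the Game level, it opens the Matting level.
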(event `self.K2_OnLogout`
  (params (ExitingController :type "Controller Object Reference"))
  (`|ExecutionSequence`
    (:`then_0`
      (bind _result (`/Engine/EditorBlueprintResources/StandardMacros.DecrementInt` (`self.NextPlayerNumber`))
        (:`  `
          (set `self.NextPlayerNumber` _result))))
    (:`then_1`
      (bind _returnvalue (`GameplayStatics.GetCurrentLevelName` true))
      (if (`KismetStringLibrary.NotEqual_StrStr` _returnvalue "Game")
        _
        (elif (<= (`self.NextPlayerNumber`) 0)
          (`GameplayStatics.OpenLevel` "Matting"))))))

(event `self.K2_PostLogin`
  (params (NewPlayer :type "PlayerController Object Reference"))
  (bind _nextteamid (`self.NextTeamID`))
  (bind _asbp_player_state (cast `/Game/GameAssets/BluePrint/PlayerState/BP_PlayerState` (`Controller.PlayerState` NewPlayer)))
  (`|ExecutionSequence`
    (:`then_0`
      (set `/Game/GameAssets/BluePrint/PlayerState/BP_PlayerState.PlayerNumber` (`self.NextPlayerNumber`) _asbp_player_state)
      (bind _result (`/Engine/EditorBlueprintResources/StandardMacros.IncrementInt` (`self.NextPlayerNumber`))
        (:`  `
          (set `self.NextPlayerNumber` _result))))
    (:`then_1`
      (set `/Game/GameAssets/BluePrint/PlayerState/BP_PlayerState.TeamID` (`self.NextTeamID`) _asbp_player_state)
      (`/Engine/EditorBlueprintResources/StandardMacros.IncrementInt` _nextteamid
        (:`  `
          (set `self.NextTeamID` (mod _nextteamid 2)))))))

(event `self.ReceiveTick`
  (params (DeltaSeconds :type "Float (single-precision)"))
  (bind _returnvalue (`GameplayStatics.GetGameState`))
  (`|ExecutionSequence`
    (:`then_0`
      (bind _asbp_game_state (cast `/Game/GameAssets/BluePrint/GameState/BP_GameState` _returnvalue))
      (set `self.Team1Cost` (`/Game/GameAssets/BluePrint/GameState/BP_GameState.Team1Cost` _asbp_game_state))
      (if (<= (`self.Team1Cost`) 0.0)
        (bind _asbp_game_state_2 (cast `/Game/GameAssets/BluePrint/GameState/BP_GameState` (`GameplayStatics.GetGameState`)))
        (set `/Game/GameAssets/BluePrint/GameState/BP_GameState.WonTeamID` 0 _asbp_game_state_2)))
    (:`then_1`
      (bind _asbp_game_state_3 (cast `/Game/GameAssets/BluePrint/GameState/BP_GameState` _returnvalue))
      (set `self.Team2Cost` (`/Game/GameAssets/BluePrint/GameState/BP_GameState.Team0Cost` _asbp_game_state_3))
      (if (<= (`self.Team2Cost`) 0.0)
        (bind _asbp_game_state_4 (cast `/Game/GameAssets/BluePrint/GameState/BP_GameState` (`GameplayStatics.GetGameState`)))
        (set `/Game/GameAssets/BluePrint/GameState/BP_GameState.WonTeamID` 1 _asbp_game_state_4)))))

(fn `UserConstructionScript`)