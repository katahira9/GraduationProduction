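; MattingMode is a matchmaking game mode that moves players to character selection once enough have joined.
; Each PostLogin increments a player counter, then checks whether the current level is something other than Game.
; When two or more players are counted there, it runs a ServerTravel console command to the CharacterSelect map.
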(event `self.K2_PostLogin`
  (params (NewPlayer :type "PlayerController Object Reference"))
  (`|ExecutionSequence`
    (:`then_0`
      (bind _result (`/Engine/EditorBlueprintResources/StandardMacros.IncrementInt` (`self.NextPlayerNumber`))
        (:`  `
          (set `self.NextPlayerNumber` _result))))
    (:`then_1`
      (bind _returnvalue (`GameplayStatics.GetCurrentLevelName` true))
      (if (`KismetStringLibrary.NotEqual_StrStr` _returnvalue "Game")
        (if (>= (`self.NextPlayerNumber`) 2)
          (`KismetSystemLibrary.ExecuteConsoleCommand` "ServerTravel CharacterSelect" null))))))

(event `self.ReceiveBeginPlay`)

(fn `UserConstructionScript`)