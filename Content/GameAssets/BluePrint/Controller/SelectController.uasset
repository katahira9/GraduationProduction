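; SelectController is a controller that copies the local player's team and player number from the player state into the game instance.
; On every Tick, only on the remote (non-authority) side, it checks that it owns a valid BP_PlayerState.
; It then writes TeamID and PlayerNumber into BP_GameInstance as TeamID and PlayerID, printing the team ID each time.
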(event `self.ReceiveBeginPlay`)

(event `self.ReceiveTick`
  (params (DeltaSeconds :type "Float (single-precision)"))
  (bind _playerstate (`self.PlayerState`))
  (bind _returnvalue (`self.GetOwner` _playerstate))
  (`/Engine/EditorBlueprintResources/ActorMacros.Switch Has Authority`
    (:`Remote`
      (`/Engine/EditorBlueprintResources/StandardMacros.IsValid` _playerstate
        (:`Is Valid`
          (if (== self _returnvalue)
            (cast `/Game/GameAssets/BluePrint/Controller/SelectController` _returnvalue)
            (bind _asbp_player_state (cast `/Game/GameAssets/BluePrint/PlayerState/BP_PlayerState` _playerstate))
            (bind _asbp_game_instance (cast `/Game/GameAssets/BluePrint/GameInstance/BP_GameInstance` (`GameplayStatics.GetGameInstance`)))
            (`|ExecutionSequence`
              (:`then_0`
                (bind _output_get (set `/Game/GameAssets/BluePrint/GameInstance/BP_GameInstance.TeamID` (`/Game/GameAssets/BluePrint/PlayerState/BP_PlayerState.TeamID` _asbp_player_state) _asbp_game_instance))
                (`KismetSystemLibrary.PrintString` (`KismetStringLibrary.Conv_IntToString` _output_get)))
              (:`then_1`
                (set `/Game/GameAssets/BluePrint/GameInstance/BP_GameInstance.PlayerID` (`/Game/GameAssets/BluePrint/PlayerState/BP_PlayerState.PlayerNumber` _asbp_player_state) _asbp_game_instance)))))))))

(fn `UserConstructionScript`)