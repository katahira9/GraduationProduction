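; A collection of stateless float and vector math helpers, mostly for working with angles in degrees.
; Yaw and pitch helpers return unsigned angles between two vectors flattened onto the XY and XZ planes.
; Other helpers wrap negative angles by 360, find shortest signed differences across the 0-360 seam, negate values and subtract toward zero without clamping.
; PermissionLerpFloat scales a value by Rate, but multiplies it by five within the tolerance.
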(fn `AngleTo_0-360`
  (params (DegreesAngel :type "Float (double-precision)"))
  (returns (OutAngle :type "Float (double-precision)"))
  (if (< DegreesAngel 0.0)
    (return (+ DegreesAngel 360.0))
    (else
      (return DegreesAngel))))

(fn `CalculateTheDifference_Angle0-360`
  (params (ObjectiveAngle :type "Float (double-precision)") (NowAngle :type "Float (double-precision)"))
  (returns (OutAngle :type "Float (double-precision)"))
  (bind _returnvalue (- ObjectiveAngle NowAngle))
  (if (> (`KismetMathLibrary.Abs` _returnvalue) 180.0)
    (if (< _returnvalue 0.0)
      ;[1 1 1] 今の角度が大きい時
      (return (+ ObjectiveAngle (- 360.0 NowAngle)))
      (else
        ;[1 1 1] 今の角度が小さい時
        (return (- (- ObjectiveAngle 360.0) NowAngle))))
    (else
      (return _returnvalue))))

(fn `Invers_Float`
  (params (value :type "Float (double-precision)"))
  (returns (float :type "Float (double-precision)"))
  (return (* -1 value)))

(fn `PermissionLerpFloat`
  (params (LerpValue :type "Float (double-precision)") (Rate :type "Float (double-precision)") (PermissionValue :type "Float (double-precision)"))
  (returns (OutValue :type "Float (double-precision)"))
  (if (<= (`KismetMathLibrary.Abs` LerpValue) PermissionValue)
    (return (* LerpValue 5.0))
    (else
      (return (`KismetMathLibrary.Lerp` 0.0 LerpValue Rate)))))

(fn `SubtractAccordingToCase`
  (params (OriginalValue :type "Float (double-precision)") (SubValue :type "Float (double-precision)"))
  (returns (OutValue :type "Float (double-precision)"))
  (if (< OriginalValue 0.0)
    (return (+ OriginalValue SubValue))
    (else
      (return (- OriginalValue SubValue)))))

(fn `TwoVectorsOfPitchAngleValue`
  (params (MainVector :type "Vector Structure") (SubVector :type "Vector Structure"))
  (returns (Angle :type "Float (double-precision)"))
  (return (`KismetMathLibrary.DegAcos` (`KismetMathLibrary.Dot_VectorVector` (`KismetMathLibrary.Normal` (`KismetMathLibrary.MakeVector` (.x MainVector) 0.0 (.z MainVector))) (`KismetMathLibrary.Normal` (`KismetMathLibrary.MakeVector` (.x SubVector) 0.0 (.z SubVector)))))))

(fn `TwoVectorsOfYawAngleValue`
  (params (MainVector :type "Vector Structure") (SubVector :type "Vector Structure"))
  (returns (Angle :type "Float (double-precision)"))
  (return (`KismetMathLibrary.DegAcos` (`KismetMathLibrary.Dot_VectorVector` (`KismetMathLibrary.Normal` (`KismetMathLibrary.MakeVector` (.x MainVector) (.y MainVector))) (`KismetMathLibrary.Normal` (`KismetMathLibrary.MakeVector` (.x SubVector) (.y SubVector)))))))